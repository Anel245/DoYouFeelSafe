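; Interactive metal sliding door that the player opens and closes with the Interact input.
; Overlapping the Box with BP_MyCharacter_CH enables input and opens a gate; leaving disables input and closes it.
; Each press flip-flops between playing and reversing the Open timeline, which drives the door mesh's relative location.
; Each direction plays its own sliding sound at the world origin rather than at the door.
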(event `InputAction|Interact`
  (params (Key :type "Key Structure"))
  (:`Pressed`
    (`/Engine/EditorBlueprintResources/StandardMacros.Gate` true :!label _label
      (:`Exit`
        (`/Engine/EditorBlueprintResources/StandardMacros.FlipFlop`
          (:`A`
            (`GameplayStatics.PlaySoundAtLocation` "/Game/GamingApartment/Audio/Slidingdoor/MSW_sliding_open.MSW_sliding_open" (0.0 0.0 0.0) (struct) 1.0 1.0 0.0 null null null null)
            (bind (_direction _slide) (`Timeline|open` :!label _label_2)
              (:`Update`
                (`SceneComponent.K2_SetRelativeLocation` (`self.SM_Metal_slingdoor`) _slide false false)
                (`/Engine/EditorBlueprintResources/StandardMacros.DoOnce` false :!via `Reset`))))
          (:`B`
            (`GameplayStatics.PlaySoundAtLocation` "/Game/GamingApartment/Audio/Slidingdoor/MSW_sliding_close.MSW_sliding_close" (0.0 0.0 0.0) (struct) 1.0 1.0 0.0 null null null null)
            (goto _label_2 :!via `Reverse`)))))))

(event `self.Box.OnComponentBeginOverlap`
  (params (OverlappedComponent :type "PrimitiveComponent Object Reference") (OtherActor :type "Actor Object Reference") (OtherComp :type "PrimitiveComponent Object Reference") (OtherBodyIndex :type Integer) (bFromSweep :type Boolean) (SweepResult :type "HitResult Structure (by ref)"))
  (cast `/Game/GamingApartment/Blueprints/BP_MyCharacter_CH` OtherActor)
  (`self.EnableInput` (`GameplayStatics.GetPlayerController` 0))
  (goto _label :!via `Open`))

(event `self.Box.OnComponentEndOverlap`
  (params (OverlappedComponent :type "PrimitiveComponent Object Reference") (OtherActor :type "Actor Object Reference") (OtherComp :type "PrimitiveComponent Object Reference") (OtherBodyIndex :type Integer))
  (cast `/Game/GamingApartment/Blueprints/BP_MyCharacter_CH` OtherActor)
  (`self.DisableInput` (`GameplayStatics.GetPlayerController` 0))
  (goto _label :!via `Close`))

(fn `UserConstructionScript`)