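; AC_GlassDoor is an interactive glass door that swings on its yaw axis when the player presses Interact nearby.
; A box overlap with BP_MyCharacter_CH enables input and opens a gate, and leaving disables both.
; Nested FlipFlops alternate presses between OpenDoor and CloseDoor timelines, each switching between Play and Reverse on its turns.
; Both timelines drive the door's relative rotation and reset a DoOnce on update.
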(event `InputAction|Interact`
  (params (Key :type "Key Structure"))
  (bind _door (`self.Door`))
  (:`Pressed`
    (`/Engine/EditorBlueprintResources/StandardMacros.Gate` true :!label _label
      (:`Exit`
        (`/Engine/EditorBlueprintResources/StandardMacros.FlipFlop`
          (:`A`
            (`/Engine/EditorBlueprintResources/StandardMacros.FlipFlop`
              (:`A`
                (bind (_direction _newtrack_0) (`Timeline|Open door` :!label _label_2)
                  (:`Update`
                    (`SceneComponent.K2_SetRelativeRotation` _door (`KismetMathLibrary.MakeRotator` 0.0 0.0 _newtrack_0) false false)
                    (`/Engine/EditorBlueprintResources/StandardMacros.DoOnce` false :!via `Reset`
                      (:`Completed`
                        (goto _label_2 :!via `PlayFromStart`))))))
              (:`B`
                (goto _label_2 :!via `Reverse`))))
          (:`B`
            (`/Engine/EditorBlueprintResources/StandardMacros.FlipFlop`
              (:`A`
                (bind (_direction_2 _newtrack_0_2) (`Timeline|Close door` :!label _label_3)
                  (:`Update`
                    (`SceneComponent.K2_SetRelativeRotation` _door (`KismetMathLibrary.MakeRotator` 0.0 0.0 _newtrack_0_2) false false)
                    (`/Engine/EditorBlueprintResources/StandardMacros.DoOnce` false :!via `Reset`
                      (:`Completed`
                        (goto _label_3 :!via `PlayFromStart`))))))
              (:`B`
                (goto _label_3 :!via `Reverse`)))))))))

(event `self.Box collision.OnComponentBeginOverlap`
  (params (OverlappedComponent :type "PrimitiveComponent Object Reference") (OtherActor :type "Actor Object Reference") (OtherComp :type "PrimitiveComponent Object Reference") (OtherBodyIndex :type Integer) (bFromSweep :type Boolean) (SweepResult :type "HitResult Structure (by ref)"))
  (cast `/Game/GamingApartment/Blueprints/BP_MyCharacter_CH` OtherActor)
  (`self.EnableInput` (`GameplayStatics.GetPlayerController` 0))
  (goto _label :!via `Open`))

(event `self.Box collision.OnComponentEndOverlap`
  (params (OverlappedComponent :type "PrimitiveComponent Object Reference") (OtherActor :type "Actor Object Reference") (OtherComp :type "PrimitiveComponent Object Reference") (OtherBodyIndex :type Integer))
  (cast `/Game/GamingApartment/Blueprints/BP_MyCharacter_CH` OtherActor)
  (`self.DisableInput` (`GameplayStatics.GetPlayerController` 0))
  (goto _label :!via `Close`))

(fn `UserConstructionScript`)