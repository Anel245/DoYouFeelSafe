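; Interactable commode furniture with six drawers that the player slides open and shut one at a time.
; Interact line-traces a short distance from the player's first-person camera to find the drawer mesh, then compares its local Y to OpenValue to choose direction.
; A timeline lerps the drawer by that offset with a sound, while CanOpen blocks re-triggering until it finishes.
; Reset snaps all drawers back to hard-coded positions.
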(event `/Game/Devs/Mert/Blueprints/Player/Interfaces/InteractionInterface.Interact`
  (bind _returnvalue (`self.K2_GetActorLocation`))
  (bind _openvalue (`self.OpenValue`))
  (bind (_relativelocation_x _relativelocation_y _relativelocation_z) (`KismetMathLibrary.BreakVector` (`SceneComponent.RelativeLocation` (`self.Static Mesh ref`))))
  (bind _asbp_player_character_mert (cast `/Game/Devs/Mert/Blueprints/Player/BP_PlayerCharacterMert` (`GameplayStatics.GetPlayerCharacter` 0)))
  (if (`self.CanOpen`)
    (set `self.CanOpen` false)
    (set `/Game/Devs/Mert/Blueprints/Player/BP_PlayerCharacterMert.Interacting` true _asbp_player_character_mert)
    (bind _firstpersoncamera (`/Game/Devs/Mert/Blueprints/Player/BP_PlayerCharacterMert.FirstPersonCamera` _asbp_player_character_mert))
    (bind _returnvalue_2 (`SceneComponent.K2_GetComponentLocation` _firstpersoncamera))
    (bind (_outhit _returnvalue_3) (`KismetSystemLibrary.LineTraceSingleForObjects` :`Start` _returnvalue_2 :`End` (+ _returnvalue_2 (* (`KismetMathLibrary.GetForwardVector` (`SceneComponent.K2_GetComponentRotation` _firstpersoncamera)) (`KismetMathLibrary.Conv_DoubleToVector` 150.0))) :`ObjectTypes` (`|MakeArray` "ObjectTypeQuery2" :!type "EObjectTypeQuery Enum") :`bIgnoreSelf` false))
    (if _returnvalue_3
      (bind _asstatic_mesh_component (cast `StaticMeshComponent` (`.HitComponent` (`GameplayStatics.BreakHitResult` _outhit))))
      (set `self.Static Mesh ref` _asstatic_mesh_component)
      (bind (_relativelocation_x_2 _relativelocation_y_2) (`KismetMathLibrary.BreakVector` (`SceneComponent.RelativeLocation` _asstatic_mesh_component)))
      (if (>= _relativelocation_y_2 (`self.OpenValue`))
        (`GameplayStatics.PlaySoundAtLocation` "/Game/Devs/Mert/Sounds/Environment/SlidingDoorClose.SlidingDoorClose" _returnvalue (struct) 1.0 1.0 0.2 null null null null)
        (set `self.OpenLocation` (`KismetMathLibrary.MakeVector` _relativelocation_x _relativelocation_y _relativelocation_z))
        (set `self.CloseLocation` (`KismetMathLibrary.MakeVector` _relativelocation_x (- _relativelocation_y _openvalue) _relativelocation_z))
        (bind (_direction _drawer) (`Timeline|Timeline` :!via `PlayFromStart`)
          (:`Update`
            (`SceneComponent.K2_SetRelativeLocation` (`self.Static Mesh ref`) (`KismetMathLibrary.VLerp` (`self.OpenLocation`) (`self.CloseLocation`) _drawer) false false))
          (:`Finished`
            (set `self.CanOpen` true)))
        (else
          (`GameplayStatics.PlaySoundAtLocation` "/Game/Devs/Mert/Sounds/Environment/SlidingDoorOpen.SlidingDoorOpen" _returnvalue (struct) 1.0 1.0 0.2 null null null null)
          (set `self.OpenLocation` (`KismetMathLibrary.MakeVector` _relativelocation_x _relativelocation_y _relativelocation_z))
          (set `self.CloseLocation` (`KismetMathLibrary.MakeVector` _relativelocation_x (+ _relativelocation_y _openvalue) _relativelocation_z))
          (bind (_direction_2 _drawer_2) (`Timeline|Drawer TL` :!via `PlayFromStart`)
            (:`Update`
              (`SceneComponent.K2_SetRelativeLocation` (`self.Static Mesh ref`) (`KismetMathLibrary.VLerp` (`self.OpenLocation`) (`self.CloseLocation`) _drawer_2) false false))
            (:`Finished`
              (set `self.CanOpen` true)))))
      (else
        (set `self.CanOpen` true)))))

(event `Reset`
  (`SceneComponent.K2_SetRelativeLocation` (`self.SM_Classic_Commode_Drawer_1`) (39.276127 1.137094 17.183462) false false)
  (`SceneComponent.K2_SetRelativeLocation` (`self.SM_Classic_Commode_Drawer_1_1`) (39.276127 1.137094 38.984615) false false)
  (`SceneComponent.K2_SetRelativeLocation` (`self.SM_Classic_Commode_Drawer_1_2`) (39.276127 1.137094 60.912491) false false)
  (`SceneComponent.K2_SetRelativeLocation` (`self.SM_Classic_Commode_Drawer_1_3`) (-39.710991 1.137094 17.183462) false false)
  (`SceneComponent.K2_SetRelativeLocation` (`self.SM_Classic_Commode_Drawer_1_4`) (-39.710991 1.137094 38.984615) false false)
  (`SceneComponent.K2_SetRelativeLocation` (`self.SM_Classic_Commode_Drawer_1_5`) (-39.710991 1.137094 60.912491) false false))

(fn `UserConstructionScript`)