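; BP_Door_2sided is an interactable double door that can be padlocked and opened with the player's key.
; Interact flags the player as interacting, then either toggles the door or, if locked, checks HasKey to play the padlock animation and unlock, or a locked sound.
; FlipFlops play or reverse a yaw timeline per leaf, with sounds.
; The Interactible flag blocks re-triggering until movement finishes.
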(event `/Game/Devs/Mert/Blueprints/Player/Interfaces/InteractionInterface.Interact`
  (bind _returnvalue (`self.K2_GetActorLocation`))
  (bind _returnvalue_2 (`self.K2_GetActorLocation`))
  (if (`self.Interactible`)
    (bind _asbp_player_character_mert_1 (cast `/Game/Devs/Mert/Meshes/AnimatedPistol/source/Animations/BP_PlayerCharacterMert1` (`GameplayStatics.GetPlayerCharacter` 0)))
    (set `/Game/Devs/Mert/Meshes/AnimatedPistol/source/Animations/BP_PlayerCharacterMert1.Interacting` true _asbp_player_character_mert_1)
    (`KismetSystemLibrary.Delay` 0.2)
    (if (`self.Unlocked`)
      (if (`self.Interactible`) :!label _label
        (set `self.Interactible` false)
        (`|ExecutionSequence`
          (:`then_0`
            (`/Engine/EditorBlueprintResources/StandardMacros.FlipFlop`
              (:`A`
                (`GameplayStatics.PlaySoundAtLocation` "/Game/Devs/Mert/Sounds/Environment/DoorLockOpening.DoorLockOpening" _returnvalue (struct) 1.0 1.0 0.0 null null null null)
                (bind (_direction _dooropen) (`Timeline|Timeline_1` :!label _label_2)
                  (:`Update`
                    (`SceneComponent.K2_SetRelativeRotation` (`self.Door_2sided_L`) (`KismetMathLibrary.MakeRotator` 0.0 0.0 _dooropen) false false))
                  (:`Finished`
                    (set `self.Interactible` true :!label _label_3))))
              (:`B`
                (goto _label_2 :!via `Reverse`))))
          (:`then_1`
            (`/Engine/EditorBlueprintResources/StandardMacros.FlipFlop`
              (:`A`
                (bind (_direction_2 _dooropen_2) (`Timeline|Timeline_0` :!label _label_4)
                  (:`Update`
                    (`SceneComponent.K2_SetRelativeRotation` (`self.Door_2sided_R`) (`KismetMathLibrary.MakeRotator` 0.0 0.0 _dooropen_2) false false))
                  (:`Finished`
                    (goto _label_3))))
              (:`B`
                (`|ExecutionSequence`
                  (:`then_0`
                    (goto _label_4 :!via `Reverse`))
                  (:`then_1`
                    (`KismetSystemLibrary.Delay` 1.6)
                    (`GameplayStatics.PlaySoundAtLocation` "/Game/Devs/Mert/Sounds/Environment/DoorCloseSound.DoorCloseSound" _returnvalue (struct) 1.0 1.0 0.0 null null null null))))))))
      (else
        (bind _outactors (`GameplayStatics.GetAllActorsOfClass` "/Game/Devs/Mert/Meshes/AnimatedPistol/source/Animations/BP_PlayerCharacterMert1.BP_PlayerCharacterMert1_C"))
        (if (`/Game/Devs/Mert/Meshes/AnimatedPistol/source/Animations/BP_PlayerCharacterMert1.HasKey` (`|GetArrayItem` _outactors))
          (`GameplayStatics.PlaySoundAtLocation` "/Game/Devs/Mert/Sounds/Environment/DoorLockOpening.DoorLockOpening" _returnvalue_2 (struct) 1.0 1.0 0.0 null null null null)
          (`SkeletalMeshComponent.PlayAnimation` (`self.Padlock`) "/Game/Devs/Mert/Meshes/PadLock/source/padlock_Padlock_Anim.padlock_Padlock_Anim" false)
          (`KismetSystemLibrary.Delay` 4.0)
          (`SceneComponent.SetVisibility` (`self.Padlock`) false false)
          (set `self.Unlocked` true)
          (goto _label)
          (else
            (`GameplayStatics.PlaySoundAtLocation` "/Game/Devs/Mert/Sounds/Environment/DoorLocked.DoorLocked" _returnvalue_2 (struct) 1.0 1.0 0.0 null null null null)
            (set `self.Interactible` false)
            (`KismetSystemLibrary.Delay` 0.7)
            (set `self.Interactible` true)))))))

(fn `UserConstructionScript`)