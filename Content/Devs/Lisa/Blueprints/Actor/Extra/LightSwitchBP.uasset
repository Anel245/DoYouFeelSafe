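; LightSwitchBP is a light switch actor that toggles its matching lights when interacted with.
; On BeginPlay it gathers every LightBP actor in the level into LightArray.
; Its Interact event loops through that cached array and calls ToggleLightsMessage on each light whose LightIndex equals the switch's own, so a shared index links one switch to any number of lights.
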(event `self.ReceiveBeginPlay`
  (bind _outactors (`GameplayStatics.GetAllActorsOfClass` "/Game/Devs/Lisa/Blueprints/Actor/Extra/LightBP.LightBP_C"))
  (for _array_element _outactors
    (`KismetArrayLibrary.Array_Add` (`self.LightArray`) _array_element)))

(event `/Game/Devs/Mert/Blueprints/Player/Interfaces/InteractionInterface.Interact`
  (for _array_element (`self.LightArray`)
    (if (== (`/Game/Devs/Lisa/Blueprints/Actor/Extra/LightBP.LightIndex` _array_element) (`self.LightIndex`))
      (message `/Game/Devs/Lisa/Blueprints/Interface/LightsInterface.ToggleLights` _array_element))))

(fn `UserConstructionScript`)