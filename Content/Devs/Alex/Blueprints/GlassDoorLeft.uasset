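; Left glass door actor that the player can open and close, swinging away from whichever side they stand on, with randomly pitched sounds.
; Front and back box overlaps track the player and start delayed polling loops that consume the Triggered flag set by Interact.
; Timelines lerp the door's yaw from its current angle.
; EnemyEntity1 overlaps swing it open after a delay, and Reset snaps it shut.
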(event `self.BoxForward.OnComponentEndOverlap`
  (params (OverlappedComponent :type "PrimitiveComponent Object Reference") (OtherActor :type "Actor Object Reference") (OtherComp :type "PrimitiveComponent Object Reference") (OtherBodyIndex :type Integer))
  ;[1 1 1] Collision End
  (cast `/Game/Devs/Mert/Blueprints/Player/BP_PlayerCharacterMert` OtherActor)
  (set `self.AtDoorFront` false))

(event `Reset`
  ;[1 1 1] Reset
  (`SceneComponent.K2_SetRelativeRotation` :`self` (`self.Door`))
  (set `self.DoorOpen` false))

(event `/Game/Devs/Mert/Blueprints/Player/Interfaces/InteractionInterface.Interact`
  ;[1 1 1] Player Interact
  (bind _asbp_player_character_mert (cast `/Game/Devs/Mert/Blueprints/Player/BP_PlayerCharacterMert` (`GameplayStatics.GetPlayerCharacter` 0)))
  (if (`self.Interactible`)
    (`|ExecutionSequence`
      (:`then_0`
        (if (`self.AtDoorFront`)
          (set `/Game/Devs/Mert/Blueprints/Player/BP_PlayerCharacterMert.Interacting` true _asbp_player_character_mert :!label _label)
          (set `self.Interactible` false)
          (set `self.Triggered` true)))
      (:`then_1`
        (if (`self.AtDoorBack`)
          (goto _label))))))

(event `self.BoxBehind.OnComponentEndOverlap`
  (params (OverlappedComponent :type "PrimitiveComponent Object Reference") (OtherActor :type "Actor Object Reference") (OtherComp :type "PrimitiveComponent Object Reference") (OtherBodyIndex :type Integer))
  ;[1 1 1] Collision End
  (cast `/Game/Devs/Mert/Blueprints/Player/BP_PlayerCharacterMert` OtherActor)
  (set `self.AtDoorBack` false))

(event `DoorUsableFront`
  (bind _returnvalue (`KismetMathLibrary.RandomFloatInRange` 0.9 1.1))
  ;[1 1 1] Player Open Door Front
  (if (`self.Triggered`) :!label _label_2
    (set `self.Triggered` false)
    (if (`self.DoorOpen`)
      (`|ExecutionSequence`
        (:`then_0`
          (bind (_direction _door_track) (`Timeline|Timeline_4` :!via `PlayFromStart`)
            (:`Update`
              (bind _returnvalue_2 (`KismetMathLibrary.Lerp` (`self.CurrentAngle`) 0.0 _door_track))
              (`SceneComponent.K2_SetRelativeRotation` (`self.Door`) (`KismetMathLibrary.MakeRotator` 0.0 0.0 _returnvalue_2) false false)
              (set `self.CurrentAngle` _returnvalue_2)
              (set `self.Triggered` false :!label _label_3)
              (`self.DoorUsableFront`))
            (:`Finished`
              (set `self.DoorOpen` false)
              (set `self.Interactible` true))))
        (:`then_1`
          (`GameplayStatics.PlaySoundAtLocation` "/Game/Devs/Mert/Sounds/Environment/DoorClose.DoorClose" (`self.K2_GetActorLocation`) (struct) 1.0 _returnvalue 0.0 null null null null)))
      (else
        (`|ExecutionSequence`
          (:`then_0`
            (bind (_direction_2 _door_track_2) (`Timeline|Timeline_3` :!via `PlayFromStart`)
              (:`Update`
                (bind _returnvalue_3 (`KismetMathLibrary.Lerp` (`self.CurrentAngle`) -80.0 _door_track_2))
                (`SceneComponent.K2_SetRelativeRotation` (`self.Door`) (`KismetMathLibrary.MakeRotator` 0.0 0.0 _returnvalue_3) false false)
                (set `self.CurrentAngle` _returnvalue_3)
                (goto _label_3))
              (:`Finished`
                (set `self.DoorOpen` true)
                (set `self.Interactible` true))))
          (:`then_1`
            (`GameplayStatics.PlaySoundAtLocation` "/Game/Devs/Mert/Sounds/Environment/DoorOpen.DoorOpen" (`self.K2_GetActorLocation`) (struct) 1.0 _returnvalue 0.3 null null null null)))))
    (else
      (`KismetSystemLibrary.Delay` 0.2)
      (if (`self.AtDoorFront`)
        (goto _label_2)))))

(event `self.BoxForward.OnComponentBeginOverlap`
  (params (OverlappedComponent :type "PrimitiveComponent Object Reference") (OtherActor :type "Actor Object Reference") (OtherComp :type "PrimitiveComponent Object Reference") (OtherBodyIndex :type Integer) (bFromSweep :type Boolean) (SweepResult :type "HitResult Structure (by ref)"))
  (`|ExecutionSequence`
    (:`then_0`
      ;[1 1 1] Player Open Door Front
      (cast `/Game/Devs/Mert/Blueprints/Player/BP_PlayerCharacterMert` OtherActor)
      (set `self.AtDoorFront` true)
      (goto _label_2))
    (:`then_1`
      ;[1 1 1] AI Open Door
      (cast `/Game/Devs/Mert/Blueprints/Enemies/EnemyEntity1` OtherActor)
      (if (`self.DoorOpen`)
        (`KismetSystemLibrary.Delay` 4.0)
        (bind (_direction _door_track) (`Timeline|Timeline_1` :!via `PlayFromStart`)
          (:`Update`
            (bind _returnvalue (`KismetMathLibrary.Lerp` (`self.CurrentAngle`) -80.0 _door_track))
            (`SceneComponent.K2_SetRelativeRotation` (`self.Door`) (`KismetMathLibrary.MakeRotator` 0.0 0.0 _returnvalue) false false)
            (set `self.CurrentAngle` _returnvalue)))
        (else
          (`KismetSystemLibrary.Delay` 8.0)
          (bind (_direction_2 _door_track_2) (`Timeline|Timeline` :!via `PlayFromStart`)
            (:`Update`
              (bind _returnvalue_2 (`KismetMathLibrary.Lerp` (`self.CurrentAngle`) -80.0 _door_track_2))
              (`SceneComponent.K2_SetRelativeRotation` (`self.Door`) (`KismetMathLibrary.MakeRotator` 0.0 0.0 _returnvalue_2) false false)
              (set `self.CurrentAngle` _returnvalue_2)))))
      (set `self.DoorOpen` true))))

(event `DoorUsableBack`
  (bind _returnvalue (`KismetMathLibrary.RandomFloatInRange` 0.9 1.1))
  ;[1 1 1] Player Open Door Behind
  (if (`self.Triggered`) :!label _label_4
    (set `self.Triggered` false)
    (if (`self.DoorOpen`)
      (`|ExecutionSequence`
        (:`then_0`
          (bind (_direction _door_track) (`Timeline|Timeline_6` :!via `PlayFromStart`)
            (:`Update`
              (bind _returnvalue_2 (`KismetMathLibrary.Lerp` (`self.CurrentAngle`) 0.0 _door_track))
              (`SceneComponent.K2_SetRelativeRotation` (`self.Door`) (`KismetMathLibrary.MakeRotator` 0.0 0.0 _returnvalue_2) false false)
              (set `self.CurrentAngle` _returnvalue_2))
            (:`Finished`
              (set `self.DoorOpen` false)
              (set `self.Interactible` true)
              (set `self.Triggered` false :!label _label_5)
              (`self.DoorUsableBack`))))
        (:`then_1`
          (`GameplayStatics.PlaySoundAtLocation` "/Game/Devs/Mert/Sounds/Environment/DoorClose.DoorClose" (`self.K2_GetActorLocation`) (struct) 1.0 _returnvalue 0.0 null null null null)))
      (else
        (`|ExecutionSequence`
          (:`then_0`
            (bind (_direction_2 _door_track_2) (`Timeline|Timeline_5` :!via `PlayFromStart`)
              (:`Update`
                (bind _returnvalue_3 (`KismetMathLibrary.Lerp` (`self.CurrentAngle`) 80.0 _door_track_2))
                (`SceneComponent.K2_SetRelativeRotation` (`self.Door`) (`KismetMathLibrary.MakeRotator` 0.0 0.0 _returnvalue_3) false false)
                (set `self.CurrentAngle` _returnvalue_3))
              (:`Finished`
                (set `self.DoorOpen` true)
                (set `self.Interactible` true)
                (goto _label_5))))
          (:`then_1`
            (`GameplayStatics.PlaySoundAtLocation` "/Game/Devs/Mert/Sounds/Environment/DoorOpen.DoorOpen" (`self.K2_GetActorLocation`) (struct) 1.0 _returnvalue 0.3 null null null null)))))
    (else
      (`KismetSystemLibrary.Delay` 0.2)
      (if (`self.AtDoorBack`)
        (goto _label_4)))))

(event `self.BoxBehind.OnComponentBeginOverlap`
  (params (OverlappedComponent :type "PrimitiveComponent Object Reference") (OtherActor :type "Actor Object Reference") (OtherComp :type "PrimitiveComponent Object Reference") (OtherBodyIndex :type Integer) (bFromSweep :type Boolean) (SweepResult :type "HitResult Structure (by ref)"))
  (`|ExecutionSequence`
    (:`then_0`
      ;[1 1 1] Player Open Door Behind
      (cast `/Game/Devs/Mert/Blueprints/Player/BP_PlayerCharacterMert` OtherActor)
      (set `self.AtDoorBack` true)
      (goto _label_4))
    (:`then_1`
      ;[1 1 1] AI Open Door
      (cast `/Game/Devs/Mert/Blueprints/Enemies/EnemyEntity1` OtherActor)
      (if (`self.DoorOpen`)
        (`KismetSystemLibrary.Delay` 4.0)
        (bind (_direction _door_track) (`Timeline|Timeline_2` :!via `PlayFromStart`)
          (:`Update`
            (bind _returnvalue (`KismetMathLibrary.Lerp` (`self.CurrentAngle`) 80.0 _door_track))
            (`SceneComponent.K2_SetRelativeRotation` (`self.Door`) (`KismetMathLibrary.MakeRotator` 0.0 0.0 _returnvalue) false false)
            (set `self.CurrentAngle` _returnvalue)))
        (else
          (`KismetSystemLibrary.Delay` 8.0)
          (bind (_direction_2 _door_track_2) (`Timeline|Timeline_0` :!via `PlayFromStart`)
            (:`Update`
              (bind _returnvalue_2 (`KismetMathLibrary.Lerp` (`self.CurrentAngle`) 80.0 _door_track_2))
              (`SceneComponent.K2_SetRelativeRotation` (`self.Door`) (`KismetMathLibrary.MakeRotator` 0.0 0.0 _returnvalue_2) false false)
              (set `self.CurrentAngle` _returnvalue_2)))))
      (set `self.DoorOpen` true))))

(fn `UserConstructionScript`)