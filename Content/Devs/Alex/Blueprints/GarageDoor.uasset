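; Garage door actor that swings open and closed on player interaction or when an EnemyEntity1 passes through its box trigger.
; Interact uses a FlipFlop to play or reverse a yaw timeline with sounds, locking interaction until it finishes and flagging the player as interacting.
; Enemy overlaps drive separate begin and end timelines, sharing the DoorOpen flag with the player path but not its FlipFlop state.
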(event `/Game/Devs/Mert/Blueprints/Player/Interfaces/InteractionInterface.Interact`
  (bind _returnvalue (`self.K2_GetActorLocation`))
  (if (`self.Interactible`)
    (set `self.Interactible` false)
    (bind _asbp_player_character_mert (cast `/Game/Devs/Mert/Blueprints/Player/BP_PlayerCharacterMert` (`GameplayStatics.GetPlayerCharacter` 0)))
    (set `/Game/Devs/Mert/Blueprints/Player/BP_PlayerCharacterMert.Interacting` true _asbp_player_character_mert)
    (`KismetSystemLibrary.Delay` 0.2)
    (`/Engine/EditorBlueprintResources/StandardMacros.FlipFlop`
      (:`A`
        (set `self.DoorOpen` true)
        (`GameplayStatics.PlaySoundAtLocation` "/Game/Devs/Mert/Sounds/Environment/DoorOpenSound.DoorOpenSound" _returnvalue (struct) 0.8 1.0 0.0 null null null null)
        (bind (_direction _door_track) (`Timeline|OpenDoor` :!label _label)
          (:`Update`
            (`SceneComponent.K2_SetRelativeRotation` (`self.Door`) (`KismetMathLibrary.MakeRotator` 0.0 0.0 (`KismetMathLibrary.Lerp` 0.0 85.0 _door_track)) false false))
          (:`Finished`
            (set `self.Interactible` true))))
      (:`B`
        (set `self.DoorOpen` false)
        (`|ExecutionSequence`
          (:`then_0`
            (goto _label :!via `Reverse`))
          (:`then_1`
            (`KismetSystemLibrary.Delay` 0.65)
            (`GameplayStatics.PlaySoundAtLocation` "/Game/Devs/Mert/Sounds/Environment/DoorCloseSound.DoorCloseSound" _returnvalue (struct) 1.0 1.0 0.0 null null null null)))))
    (else
      (set `/Game/Devs/Mert/Blueprints/Player/BP_PlayerCharacterMert.Interacting` false _asbp_player_character_mert))))

(event `self.Box.OnComponentBeginOverlap`
  (params (OverlappedComponent :type "PrimitiveComponent Object Reference") (OtherActor :type "Actor Object Reference") (OtherComp :type "PrimitiveComponent Object Reference") (OtherBodyIndex :type Integer) (bFromSweep :type Boolean) (SweepResult :type "HitResult Structure (by ref)"))
  ;[1 1 1] AI Open/Close Door
  (cast `/Game/Devs/Mert/Blueprints/Enemies/EnemyEntity1` OtherActor)
  (if (not (`self.DoorOpen`))
    (bind (_direction _door_track) (`Timeline|Timeline`)
      (:`Update`
        (`SceneComponent.K2_SetRelativeRotation` (`self.Door`) (`KismetMathLibrary.MakeRotator` 0.0 0.0 (`KismetMathLibrary.Lerp` 0.0 95.0 _door_track)) false false))
      (:`Finished`
        (set `self.DoorOpen` true)))))

(event `self.Box.OnComponentEndOverlap`
  (params (OverlappedComponent :type "PrimitiveComponent Object Reference") (OtherActor :type "Actor Object Reference") (OtherComp :type "PrimitiveComponent Object Reference") (OtherBodyIndex :type Integer))
  ;[1 1 1] AI Open/Close Door
  (cast `/Game/Devs/Mert/Blueprints/Enemies/EnemyEntity1` OtherActor)
  (if (`self.DoorOpen`)
    (bind (_direction _door_track) (`Timeline|Timeline_0`)
      (:`Update`
        (`SceneComponent.K2_SetRelativeRotation` (`self.Door`) (`KismetMathLibrary.MakeRotator` 0.0 0.0 (`KismetMathLibrary.Lerp` 0.0 95.0 _door_track)) false false))
      (:`Finished`
        (set `self.DoorOpen` false)
        (`GameplayStatics.PlaySoundAtLocation` "/Game/Devs/Mert/Sounds/Environment/DoorCloseSound.DoorCloseSound" (`self.K2_GetActorLocation`) (struct) 1.0 1.0 0.0 null null null null)))))

(fn `UserConstructionScript`)