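; EntranceDoor is an interactable door Blueprint that tells the player it is locked and contains no opening logic.
; Interact casts the player to BP_PlayerCharacterMert and, while Interactible is true, flags the player as Interacting.
; KeyCount selects the W_LockedStill widget when keys are held, otherwise W_Locked, and calls its Opacity function.
; A delay then sets Interactible true, though nothing here sets it false.
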(event `/Game/Devs/Mert/Blueprints/Player/Interfaces/InteractionInterface.Interact`
  ;[1 1 1] Player Interact
  (bind _asbp_player_character_mert (cast `/Game/Devs/Mert/Blueprints/Player/BP_PlayerCharacterMert` (`GameplayStatics.GetPlayerCharacter` 0)))
  (if (`self.Interactible`)
    (set `/Game/Devs/Mert/Blueprints/Player/BP_PlayerCharacterMert.Interacting` true _asbp_player_character_mert)
    (if (> (`/Game/Devs/Mert/Blueprints/Player/BP_PlayerCharacterMert.KeyCount` _asbp_player_character_mert) 0)
      (bind _returnvalue (`|CreateWidget` "/Game/Devs/Mert/Blueprints/Player/Widgets/W_Dialogue/W_LockedStill.W_LockedStill_C"))
      (`UserWidget.AddToViewport` _returnvalue 0)
      (`/Game/Devs/Mert/Blueprints/Player/Widgets/W_Dialogue/W_LockedStill.Opacity` _returnvalue)
      (`KismetSystemLibrary.Delay` 6.0)
      (set `self.Interactible` true)
      (else
        (bind _returnvalue_2 (`|CreateWidget` "/Game/Devs/Mert/Blueprints/Player/Widgets/W_Dialogue/W_Locked.W_Locked_C"))
        (`UserWidget.AddToViewport` _returnvalue_2 0)
        (`/Game/Devs/Mert/Blueprints/Player/Widgets/W_Dialogue/W_Locked.Opacity` _returnvalue_2)
        (`KismetSystemLibrary.Delay` 4.0)
        (set `self.Interactible` true)))))

(fn `UserConstructionScript`)