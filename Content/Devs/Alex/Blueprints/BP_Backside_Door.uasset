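; BP_Backside_Door is a sliding door that the player toggles through interaction and that enemies open automatically.
; A timeline slides the door, playing forward to open and reversing to close.
; Interact locks out re-use until the timeline finishes, flags the player as interacting, and toggles the door with sound after a brief delay.
; EnemyEntity1 or EnemyMinionEntity1 overlapping the box opens it silently, while Reset closes it silently.
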(event `self.Box.OnComponentBeginOverlap`
  (params (OverlappedComponent :type "PrimitiveComponent Object Reference") (OtherActor :type "Actor Object Reference") (OtherComp :type "PrimitiveComponent Object Reference") (OtherBodyIndex :type Integer) (bFromSweep :type Boolean) (SweepResult :type "HitResult Structure (by ref)"))
  (`|ExecutionSequence`
    (:`then_0`
      (cast `/Game/Devs/Mert/Blueprints/Enemies/EnemyEntity1` OtherActor))
    (:`then_1`
      (cast `/Game/Devs/Mert/Blueprints/Enemies/EnemyMinionEntity1` OtherActor)))
  (set `self.DoorOpen` true)
  (bind (_direction _slidinganimation) (`Timeline|Door Slide TL` :!label _label)
    (:`Update`
      (`SceneComponent.K2_SetRelativeLocation` (`self.Sliding_Door`) _slidinganimation false false))
    (:`Finished`
      (set `self.Interactible` true))))

(event `/Game/Devs/Mert/Blueprints/Player/Interfaces/InteractionInterface.Interact`
  (bind _returnvalue (`self.K2_GetActorLocation`))
  (if (`self.Interactible`)
    (set `self.Interactible` false)
    (bind _asbp_player_character_mert (cast `/Game/Devs/Mert/Blueprints/Player/BP_PlayerCharacterMert` (`GameplayStatics.GetPlayerCharacter` 0)))
    (set `/Game/Devs/Mert/Blueprints/Player/BP_PlayerCharacterMert.Interacting` true _asbp_player_character_mert)
    (`KismetSystemLibrary.Delay` 0.2)
    (if (`self.DoorOpen`)
      (`GameplayStatics.PlaySoundAtLocation` "/Game/Devs/Mert/Sounds/Environment/SlidingDoorClose.SlidingDoorClose" _returnvalue (struct) 1.0 1.0 0.0 null null null null)
      (set `self.DoorOpen` false :!label _label_2)
      (goto _label :!via `Reverse`)
      (else
        (set `self.DoorOpen` true)
        (`GameplayStatics.PlaySoundAtLocation` "/Game/Devs/Mert/Sounds/Environment/SlidingDoorOpen.SlidingDoorOpen" _returnvalue (struct) 0.8 1.0 0.0 null null null null)
        (goto _label)))))

(event `Reset`
  (goto _label_2))

(fn `UserConstructionScript`)