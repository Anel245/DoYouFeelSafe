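; Interactible double door for the livingroom, locked by an animated padlock that consumes one player key to open.
; Interact checks the player's loop, tutorial and gun state, showing a hint widget or guidance text when blocked.
; Once unlocked, two timelines swing the leaves apart by mirrored yaw lerps; interacting does not close them.
; Reset restores the padlock, relocks the door and reverses both timelines.
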(event `/Game/Devs/Mert/Blueprints/Player/Interfaces/InteractionInterface.Interact`
  (if (`self.Interactible`)
    (bind _asbp_player_character_mert (cast `/Game/Devs/Mert/Blueprints/Player/BP_PlayerCharacterMert` (`GameplayStatics.GetPlayerCharacter` 0)))
    (set `/Game/Devs/Mert/Blueprints/Player/BP_PlayerCharacterMert.Interacting` true _asbp_player_character_mert)
    (`KismetSystemLibrary.Delay` 0.2)
    (if (`/Game/Devs/Mert/Blueprints/Player/BP_PlayerCharacterMert.1 Loop` _asbp_player_character_mert)
      (if (`self.Unlocked`) :!label _label
        (if (`self.Interactible`) :!label _label_2
          (set `self.Interactible` false)
          (if (not (`self.DoorOpen`))
            (`|ExecutionSequence`
              (:`then_0`
                (`GameplayStatics.PlaySoundAtLocation` "/Game/Devs/Mert/Sounds/Environment/DoorLockOpening.DoorLockOpening" (`self.K2_GetActorLocation`) (struct) 1.0 1.0 0.0 null null null null)
                (set `self.DoorOpen` true)
                (bind (_direction _dooropen) (`Timeline|Timeline_1` :!label _label_3)
                  (:`Update`
                    (`SceneComponent.K2_SetRelativeRotation` (`self.Door_2sided_L`) (`KismetMathLibrary.MakeRotator` 0.0 0.0 (`KismetMathLibrary.Lerp` 0.0 (`self.OpenAngle`) _dooropen)) false false))
                  (:`Finished`
                    (set `self.Interactible` true :!label _label_4))))
              (:`then_1`
                (set `self.DoorOpen` true)
                (bind (_direction_2 _dooropen_2) (`Timeline|Timeline_0` :!label _label_5)
                  (:`Update`
                    (`SceneComponent.K2_SetRelativeRotation` (`self.Door_2sided_R`) (`KismetMathLibrary.MakeRotator` 0.0 0.0 (`KismetMathLibrary.Lerp` 0.0 (* (`self.OpenAngle`) -1.0) _dooropen_2)) false false))
                  (:`Finished`
                    (goto _label_4)))))))
        (else
          (bind _asbp_player_character_mert_2 (cast `/Game/Devs/Mert/Blueprints/Player/BP_PlayerCharacterMert` (`GameplayStatics.GetPlayerCharacter` 0)))
          (if (> (`/Game/Devs/Mert/Blueprints/Player/BP_PlayerCharacterMert.KeyCount` _asbp_player_character_mert_2) 0)
            (`/Engine/EditorBlueprintResources/StandardMacros.DoOnce` false :!label _label_6
              (:`Completed`
                (set `/Game/Devs/Mert/Blueprints/Player/BP_PlayerCharacterMert.KeyCount` (- (`/Game/Devs/Mert/Blueprints/Player/BP_PlayerCharacterMert.KeyCount` _asbp_player_character_mert_2) 1) _asbp_player_character_mert_2)
                (`SkeletalMeshComponent.PlayAnimation` (`self.Padlock`) "/Game/Devs/Mert/Meshes/PadLock/source/padlock_Padlock_Anim.padlock_Padlock_Anim" false)
                (`GameplayStatics.PlaySound2D` "/Game/Devs/Mert/Sounds/Player-Footsteps/PickUp.PickUp" 1.0 1.0 0.0 null null false)
                (`KismetSystemLibrary.Delay` 4.0)
                (`SceneComponent.SetVisibility` (`self.Padlock`) false false)
                (set `self.Unlocked` true)
                (goto _label_2)))
            (elif (not (`self.Unlocked`))
              (`GameplayStatics.PlaySoundAtLocation` "/Game/Devs/Mert/Sounds/Environment/DoorLocked.DoorLocked" (`self.K2_GetActorLocation`) (struct) 1.0 1.0 0.0 null null null null)
              (set `self.Interactible` false)
              (`KismetSystemLibrary.Delay` 0.7)
              (set `self.Interactible` true)
              (if (`/Game/Devs/Mert/Blueprints/Player/BP_PlayerCharacterMert.Tutorial` _asbp_player_character_mert_2)
                (bind _returnvalue (`|CreateWidget` "/Game/Devs/Mert/Blueprints/Player/Widgets/W_Dialogue/W_NeedKey.W_NeedKey_C"))
                (`UserWidget.AddToViewport` _returnvalue 0)
                (`/Game/Devs/Mert/Blueprints/Player/Widgets/W_Dialogue/W_NeedKey.Opacity` _returnvalue)
                (else
                  (set `/Game/Devs/Mert/Blueprints/Player/BP_PlayerCharacterMert.CurrentGuidance` "Find the key for the livingroom" _asbp_player_character_mert_2)))))))
      (elif (`/Game/Devs/Mert/Blueprints/Player/BP_PlayerCharacterMert.Tutorial` _asbp_player_character_mert)
        (goto _label)
        (elif (`/Game/Devs/Mert/Blueprints/Player/BP_PlayerCharacterMert.HasGun` _asbp_player_character_mert)
          (goto _label)
          (elif (`/Game/Devs/Mert/Blueprints/Player/BP_PlayerCharacterMert.3 Loop` _asbp_player_character_mert)
            (goto _label)
            (else
              (bind _returnvalue_2 (`|CreateWidget` "/Game/Devs/Mert/Blueprints/Player/Widgets/W_Dialogue/W_FindGunFirst.W_FindGunFirst_C"))
              (`UserWidget.AddToViewport` _returnvalue_2 0)
              (`/Game/Devs/Mert/Blueprints/Player/Widgets/W_Dialogue/W_FindGunFirst.Opacity` _returnvalue_2))))))))

(event `Reset`
  (`SceneComponent.SetVisibility` (`self.Padlock`) true false)
  (set `self.Unlocked` false)
  (set `self.DoorOpen` false)
  (`|ExecutionSequence`
    (:`then_0`
      (goto _label_3 :!via `Reverse`))
    (:`then_1`
      (goto _label_5 :!via `Reverse`))
    (:`then_2`
      (goto _label_6 :!via `Reset`))))

(fn `UserConstructionScript`)