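; Interactive wooden door that the player swings by holding F and turning, and that enemies can push.
; Interact polls DoorInteracting, which locks look input, rotates the door by TurnRate within OpenAngle, plays open/close sounds and frees the camera if the player keeps moving.
; EnemyEntity1 overlaps on front/back boxes wait, then swing player-opened doors to either side via timelines.
; Reset snaps the door shut.
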(event `DoorInteracting`
  (bind _returnvalue (`self.K2_GetActorLocation`))
  (bind _returnvalue_2 (`GameplayStatics.GetPlayerController` 0))
  (bind _openangle (`self.OpenAngle`))
  (bind _openangle_2 (`self.OpenAngle`))
  (bind _door (`self.Door`))
  (bind (_relativerotation_roll _relativerotation_pitch _relativerotation_yaw) (`KismetMathLibrary.BreakRotator` (`SceneComponent.RelativeRotation` (`self.Door`))))
  ;[1 1 1] Door Angle Function
  (if (`self.IsHoldingDoor`)
    (if (not (`self.WalkedAway`))
      (bind _returnvalue_3 (> (`KismetMathLibrary.VSize` (`self.GetVelocity` (stale `/Game/Devs/Mert/Blueprints/Player/Interfaces/InteractionInterface.Interact` _asbp_player_character_mert))) 0.0))
      (if _returnvalue_3
        (`|ExecutionSequence`
          (:`then_0`
            (`Controller.SetIgnoreLookInput` _returnvalue_2 true :!label _label)
            (set `self.CurrentAngle` _relativerotation_yaw)
            (if (not (== _relativerotation_yaw (`KismetMathLibrary.ClampAngle` _relativerotation_yaw _openangle_2 (* _openangle_2 -1.0))))
              (set `self.DoorOpen` true)
              (set `self.Player Opened` true)
              (`|ExecutionSequence`
                (:`then_0`
                  (if (and (> _relativerotation_yaw -0.3) (< _relativerotation_yaw 0.3))
                    (if (not (`self.Reseted`))
                      (`/Engine/EditorBlueprintResources/StandardMacros.DoOnce` true :!label _label_2
                        (:`Completed`
                          (`GameplayStatics.PlaySoundAtLocation` "/Game/Devs/Mert/Sounds/Environment/DoorClose.DoorClose" _returnvalue (struct) 1.0 1.0 0.0 null null null null)
                          (set `self.DoorOpen` false)
                          (set `self.IsHoldingDoor` false))))
                    (else
                      (`KismetSystemLibrary.Delay` 0.2)
                      (if (not (and (> _relativerotation_yaw -2.0) (< _relativerotation_yaw 2.0)))
                        (set `self.Reseted` false)
                        (goto _label_2 :!via `Reset`)))))
                (:`then_1`
                  (`SceneComponent.K2_AddLocalRotation` (`self.Door`) (`KismetMathLibrary.MakeRotator` 0.0 0.0 (* (`/Game/Devs/Mert/Blueprints/Player/BP_PlayerCharacterMert.TurnRate` (stale `/Game/Devs/Mert/Blueprints/Player/Interfaces/InteractionInterface.Interact` _asbp_player_character_mert)) (`self.Sensitivity`))) false false)
                  (`|ExecutionSequence`
                    (:`then_0`
                      (if (`self.DoorOpen`)
                        (`/Engine/EditorBlueprintResources/StandardMacros.DoOnce` false :!label _label_3
                          (:`Completed`
                            (`GameplayStatics.PlaySoundAtLocation` "/Game/Devs/Mert/Sounds/Environment/DoorOpen.DoorOpen" _returnvalue (struct) 1.0 1.0 0.0 null null null null :!label _label_4)))
                        (else
                          (`KismetSystemLibrary.Delay` 0.2)
                          (goto _label_3 :!via `Reset`))))
                    (:`then_1`
                      (if (`self.Reseted`)
                        (`/Engine/EditorBlueprintResources/StandardMacros.DoOnce` false :!label _label_5
                          (:`Completed`
                            (goto _label_4))))))))
              (elif (>= _relativerotation_yaw (`self.OpenAngle`))
                (`SceneComponent.K2_SetRelativeRotation` _door (`KismetMathLibrary.MakeRotator` 0.0 0.0 (- _openangle 1.0)) false false)
                (else
                  (`SceneComponent.K2_SetRelativeRotation` _door (`KismetMathLibrary.MakeRotator` 0.0 0.0 (+ (* _openangle -1.0) 1.0)) false false)))))
          (:`then_1`
            (`KismetSystemLibrary.Delay` 2.0)
            (if _returnvalue_3
              (if (`self.IsHoldingDoor`)
                (set `self.WalkedAway` true)
                (`Controller.ResetIgnoreLookInput` _returnvalue_2)))))
        (else
          (goto _label))))))

(event `/Game/Devs/Mert/Blueprints/Player/Interfaces/InteractionInterface.Interact`
  (bind _returnvalue (`GameplayStatics.GetPlayerController` 0))
  ;[1 1 1] Player Interact
  (bind _asbp_player_character_mert (cast `/Game/Devs/Mert/Blueprints/Player/BP_PlayerCharacterMert` (`GameplayStatics.GetPlayerCharacter` 0)))
  (set `/Game/Devs/Mert/Blueprints/Player/BP_PlayerCharacterMert.Interacting` true _asbp_player_character_mert)
  (set `self.IsHoldingDoor` true)
  (if (`PlayerController.IsInputKeyDown` _returnvalue "F") :!label _label_6
    (`KismetSystemLibrary.Delay` 0.002)
    (`self.DoorInteracting`)
    (goto _label_6)
    (else
      (set `/Game/Devs/Mert/Blueprints/Player/BP_PlayerCharacterMert.Interacting` false _asbp_player_character_mert)
      (set `self.IsHoldingDoor` false)
      (set `self.WalkedAway` false)
      (`Controller.ResetIgnoreLookInput` _returnvalue)
      (goto _label_5 :!via `Reset`))))

(event `self.BoxForward.OnComponentBeginOverlap`
  (params (OverlappedComponent :type "PrimitiveComponent Object Reference") (OtherActor :type "Actor Object Reference") (OtherComp :type "PrimitiveComponent Object Reference") (OtherBodyIndex :type Integer) (bFromSweep :type Boolean) (SweepResult :type "HitResult Structure (by ref)"))
  ;[1 1 1] AI Open/Close Door
  (cast `/Game/Devs/Mert/Blueprints/Enemies/EnemyEntity1` OtherActor)
  (if (`self.DoorOpen`)
    (`KismetSystemLibrary.Delay` 4.0)
    (if (`self.Player Opened`)
      (bind (_direction _door_track) (`Timeline|Timeline_1`)
        (:`Update`
          (`SceneComponent.K2_SetRelativeRotation` (`self.Door`) (`KismetMathLibrary.MakeRotator` 0.0 0.0 (`KismetMathLibrary.Lerp` (`self.CurrentAngle`) 80.0 _door_track)) false false)
          (set `self.DoorOpen` true :!label _label_7)
          (set `self.Player Opened` false))))
    (else
      (`KismetSystemLibrary.Delay` 8.0)
      (if (`self.Player Opened`)
        (bind (_direction_2 _door_track_2) (`Timeline|Timeline`)
          (:`Update`
            (`SceneComponent.K2_SetRelativeRotation` (`self.Door`) (`KismetMathLibrary.MakeRotator` 0.0 0.0 (`KismetMathLibrary.Lerp` (`self.CurrentAngle`) 80.0 _door_track_2)) false false)
            (goto _label_7)))))))

(event `self.BoxBehind.OnComponentBeginOverlap`
  (params (OverlappedComponent :type "PrimitiveComponent Object Reference") (OtherActor :type "Actor Object Reference") (OtherComp :type "PrimitiveComponent Object Reference") (OtherBodyIndex :type Integer) (bFromSweep :type Boolean) (SweepResult :type "HitResult Structure (by ref)"))
  ;[1 1 1] AI Open/Close Door
  (cast `/Game/Devs/Mert/Blueprints/Enemies/EnemyEntity1` OtherActor)
  (if (`self.DoorOpen`)
    (`KismetSystemLibrary.Delay` 4.0)
    (if (`self.Player Opened`)
      (bind (_direction _door_track) (`Timeline|Timeline_2`)
        (:`Update`
          (`SceneComponent.K2_SetRelativeRotation` (`self.Door`) (`KismetMathLibrary.MakeRotator` 0.0 0.0 (`KismetMathLibrary.Lerp` (`self.CurrentAngle`) -80.0 _door_track)) false false)
          (goto _label_7))))
    (else
      (`KismetSystemLibrary.Delay` 8.0)
      (if (`self.Player Opened`)
        (bind (_direction_2 _door_track_2) (`Timeline|Timeline_0`)
          (:`Update`
            (`SceneComponent.K2_SetRelativeRotation` (`self.Door`) (`KismetMathLibrary.MakeRotator` 0.0 0.0 (`KismetMathLibrary.Lerp` (`self.CurrentAngle`) -80.0 _door_track_2)) false false)
            (goto _label_7)))))))

(event `Reset`
  ;[1 1 1] Reset
  (`SceneComponent.K2_SetRelativeRotation` :`self` (`self.Door`))
  (set `self.DoorOpen` false)
  (set `self.Reseted` true))

(fn `UserConstructionScript`)