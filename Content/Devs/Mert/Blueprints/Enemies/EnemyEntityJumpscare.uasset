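; Enemy entity actor that performs two one-shot jumpscares on the player, both turning it to face them.
; RunJumpscare uses a timeline to lerp it toward a given location, playing a boom and notifying one BP_PointLight when CanSeeEnemy is true, then destroys it when finished.
; StandJumpscare plays the boom in place, waits briefly, destroys the actor and calls EnemyPlayerSee on all point lights.
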(event `Run Jumpscare`
  (params (Location :type "Vector Structure"))
  (bind (_direction _speed) (`Timeline|Run TL`)
    (:`Update`
      (`self.K2_SetActorLocation` (`KismetMathLibrary.VLerp` (`self.K2_GetActorLocation`) Location _speed))
      (bind _asbp_player_character_mert (cast `/Game/Devs/Mert/Blueprints/Player/BP_PlayerCharacterMert` (`GameplayStatics.GetPlayerPawn` 0)))
      (`self.K2_SetActorRotation` (`KismetMathLibrary.FindLookAtRotation` (`self.K2_GetActorLocation`) (`self.K2_GetActorLocation` _asbp_player_character_mert)))
      (if (`/Game/Devs/Mert/Blueprints/Player/BP_PlayerCharacterMert.CanSeeEnemy` _asbp_player_character_mert)
        (`/Engine/EditorBlueprintResources/StandardMacros.DoOnce` false
          (:`Completed`
            (`GameplayStatics.PlaySound2D` "/Game/Devs/Mert/Sounds/Entity/BoomJumpscareSound.BoomJumpscareSound" 3.0 1.0 0.4 null null false)
            (bind _returnvalue (`GameplayStatics.GetActorOfClass` "/Game/Devs/Mert/Blueprints/Environment/Static/BP_PointLight.BP_PointLight_C"))
            (`/Game/Devs/Mert/Blueprints/Environment/Static/BP_PointLight.Enemy/Player See` _returnvalue)))))
    (:`Finished`
      (`self.K2_DestroyActor`))))

(event `Stand Jumpscare`
  (bind _asbp_player_character_mert (cast `/Game/Devs/Mert/Blueprints/Player/BP_PlayerCharacterMert` (`GameplayStatics.GetPlayerPawn` 0)))
  (`self.K2_SetActorRotation` (`KismetMathLibrary.FindLookAtRotation` (`self.K2_GetActorLocation`) (`self.K2_GetActorLocation` _asbp_player_character_mert)))
  (`/Engine/EditorBlueprintResources/StandardMacros.DoOnce` false
    (:`Completed`
      (`GameplayStatics.PlaySound2D` "/Game/Devs/Mert/Sounds/Entity/BoomJumpscareSound.BoomJumpscareSound" 1.5 1.0 0.4 null null false)
      (`KismetSystemLibrary.Delay` 0.4)
      (`self.K2_DestroyActor`)
      (bind _outactors (`GameplayStatics.GetAllActorsOfClass` "/Game/Devs/Mert/Blueprints/Environment/Static/BP_PointLight.BP_PointLight_C"))
      (`/Game/Devs/Mert/Blueprints/Environment/Static/BP_PointLight.Enemy/Player See` _outactors))))

(fn `UserConstructionScript`)