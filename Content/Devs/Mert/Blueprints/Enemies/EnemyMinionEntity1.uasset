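; Minion enemy that roams randomly with heartbeat audio and chases the player once seen.
; PawnSensing starts the chase and turn-to-face loop, while a tick-driven forward trace updates visibility and triggers player vision and light reactions.
; Its stun sphere plays a scale-up timeline, then removes a player health segment, alerts EnemyEntity1 and self-destructs, or kills the player on the last segment.
; Killing it by damage increments an achievement counter.
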(event `self.ReceiveTick`
  (params (DeltaSeconds :type "Float (single-precision)"))
  (bind _cube (`self.Cube`))
  (bind _returnvalue (`SceneComponent.K2_GetComponentLocation` _cube))
  ;[1 0 0 0] Initial Tick
  (`|ExecutionSequence`
    (:`then_0`
      (if (not (`self.IsMoving`))
        (`KismetSystemLibrary.Delay` (`KismetMathLibrary.RandomFloatInRange` 3.0 6.0))
        (if (not (`self.CanSeePlayer`))
          (set `self.IsMoving` true)
          (set `CharacterMovementComponent.MaxWalkSpeed` (`self.EntityWalkSpeed`) (`self.CharacterMovement`))
          (`|AIMoveTo` self (`NavigationSystemV1.K2_GetRandomReachablePointInRadius` (`self.K2_GetActorLocation`) 1500.0 null null) null 300.0
            (:`then`
              (if (`self.IsMoving`) :!label _label
                (if (not (`self.CanSeePlayer`))
                  (`GameplayStatics.PlaySoundAtLocation` "/Game/Devs/Mert/Sounds/Entity/HeartbeatSound_Cue.HeartbeatSound_Cue" (`self.K2_GetActorLocation`) (struct) 0.1 1.0 0.0 "/Game/Devs/Mert/Sounds/Entity/EntityAttenuation.EntityAttenuation" null null null)
                  (`KismetSystemLibrary.Delay` 2.9)
                  (goto _label))))
            (:`OnSuccess`
              (set `self.IsMoving` false :!label _label_2))
            (:`OnFail`
              (goto _label_2))))))
    (:`then_1`
      (`KismetSystemLibrary.Delay` 0.2)
      (bind (_outhits _returnvalue_2) (`KismetSystemLibrary.LineTraceMultiForObjects` _returnvalue (+ _returnvalue (* (`KismetMathLibrary.GetForwardVector` (`SceneComponent.K2_GetComponentRotation` _cube)) (`KismetMathLibrary.Conv_DoubleToVector` 1000.0))) (`|MakeArray` "ObjectTypeQuery3" :!type "EObjectTypeQuery Enum")))
      (bind _asbp_player_character_mert (cast `/Game/Devs/Mert/Blueprints/Player/BP_PlayerCharacterMert` (`GameplayStatics.GetPlayerPawn` 0)))
      (if _returnvalue_2
        (set `self.CanSeePlayer` true)
        (`/Game/Devs/Mert/Blueprints/Player/BP_PlayerCharacterMert.Chromatic PlayerVision` _asbp_player_character_mert)
        (bind _outactors (`GameplayStatics.GetAllActorsOfClass` "/Game/Devs/Mert/Blueprints/Environment/Static/BP_PointLight.BP_PointLight_C"))
        (`/Game/Devs/Mert/Blueprints/Environment/Static/BP_PointLight.Enemy/Player See` _outactors)
        (else
          (set `self.CanSeePlayer` false)
          (set `self.IsMoving` false))))))

(event `self.PawnSensing.OnSeePawn`
  (params (Pawn :type "Pawn Object Reference"))
  ;[0.001892 0 1 0.1] AI Sense
  ;;[0 0 1 0] Sense Player
  (bind _asbp_player_character_mert (cast `/Game/Devs/Mert/Blueprints/Player/BP_PlayerCharacterMert` Pawn))
  (set `self.CanSeePlayer` true)
  (if (`/Game/Devs/Mert/Blueprints/Player/BP_PlayerCharacterMert.IsPlayerActive` _asbp_player_character_mert)
    (`self.ChasePlayer`)
    (`self.FacePlayer`)
    (else
      (set `self.CanSeePlayer` false)
      (set `self.IsMoving` false))))

(event `TriggerJumpscare`
  ;[0 0.9383 1 0.1] Enemy Events
  ;;[0 0.9373 1 0] Activate Player Jumpscare & Death
  (bind _asbp_player_character_mert (cast `/Game/Devs/Mert/Blueprints/Player/BP_PlayerCharacterMert` (`GameplayStatics.GetPlayerPawn` 0)))
  (if (`/Game/Devs/Mert/Blueprints/Player/BP_PlayerCharacterMert.IsPlayerActive` _asbp_player_character_mert)
    (`/Engine/EditorBlueprintResources/StandardMacros.DoOnce` false
      (:`Completed`
        (`/Game/Devs/Mert/Blueprints/Player/BP_PlayerCharacterMert.PlayerJumpscare` _asbp_player_character_mert)))))

(event `self.ReceiveAnyDamage`
  (params (Damage :type "Float (single-precision)") (DamageType :type "DamageType Object Reference") (InstigatedBy :type "Controller Object Reference") (DamageCauser :type "Actor Object Reference"))
  ;[0 0.9383 1 0.1] Enemy Events
  ;;[0 0.9373 1 0] Enemy Damaged
  (`self.FacePlayer`)
  (bind _output_get (set `self.EnemyHealth` (- (`self.EnemyHealth`) Damage)))
  (if (<= _output_get 0.0)
    (`self.K2_DestroyActor`)
    (`AudioComponent.AdjustVolume` (`self.RisingSound ref`) 0.0 0.0 "Linear")
    (`GameplayStatics.PlaySoundAtLocation` "/Game/Devs/Mert/Sounds/Environment/BassDropSound.BassDropSound" (`self.K2_GetActorLocation`) (struct) 1.0 1.0 0.0 "/Game/Devs/Mert/Sounds/Entity/EntityAttenuation.EntityAttenuation" null null null)
    ;[0.5798 0.3256 0.8021] MinionKillercounter for achievement
    (bind _outactors (`GameplayStatics.GetAllActorsOfClass` "/Game/Devs/Lisa/Blueprints/Actor/AchievementActors/MinionsKillerCounter_BP.MinionsKillerCounter_BP_C"))
    (bind _output (`|GetArrayItem` _outactors))
    (set `/Game/Devs/Lisa/Blueprints/Actor/AchievementActors/MinionsKillerCounter_BP.MinionDeathCounts` (+ (`/Game/Devs/Lisa/Blueprints/Actor/AchievementActors/MinionsKillerCounter_BP.MinionDeathCounts` _output) 1) _output)))

(event `ChasePlayer`
  ;[0.001892 0 1 0.1] AI Sense
  ;;[0 0 1 0] Following & Chasing Player
  (cast `/Game/Devs/Mert/Blueprints/Player/BP_PlayerCharacterMert` (`GameplayStatics.GetPlayerPawn` 0))
  (if (`self.CanSeePlayer`)
    (set `self.IsMoving` true)
    (set `CharacterMovementComponent.MaxWalkSpeed` (`self.EntityRunSpeed`) (`self.CharacterMovement`))
    (`|AIMoveTo` self (0.0 0.0 0.0) (`GameplayStatics.GetPlayerCharacter` 0) 175.0
      (:`then`
        (set `self.CanSeePlayer` true)
        (set `self.IsMoving` true)
        (`|ExecutionSequence`
          (:`then_0`
            (`/Engine/EditorBlueprintResources/StandardMacros.DoOnce` false :!label _label_3
              (:`Completed`
                (`KismetSystemLibrary.Delay` 0.6)
                (if (`self.IsMoving`)
                  (`GameplayStatics.PlaySoundAtLocation` "/Game/Devs/Mert/Sounds/Entity/HeartbeatSound_Cue.HeartbeatSound_Cue" (`self.K2_GetActorLocation`) (struct) 0.2 1.0 0.0 "/Game/Devs/Mert/Sounds/Entity/EntityAttenuation.EntityAttenuation" null null null)
                  (goto _label_3 :!via `Reset`)))))
          (:`then_1`
            (if (not (`/Game/Devs/Mert/Blueprints/Player/BP_PlayerCharacterMert.IsInFear` (`self.Player ref`)))
              (`KismetSystemLibrary.Delay` 2.0 :!label _label_4)
              (`/Engine/EditorBlueprintResources/StandardMacros.DoOnce` false
                (:`Completed`
                  (bind _returnvalue (`AddComponent|NODE_AddAudioComponent-1`))
                  (`AudioComponent.AdjustVolume` _returnvalue 1.0 2.0 "Linear")
                  (goto _label_4)))))))
      (:`OnFail`
        (`KismetSystemLibrary.Delay` 1.0 :!label _label_5)
        (set `self.IsMoving` false)
        (`AudioComponent.AdjustVolume` _returnvalue 1.0 0.0 "Linear")))
    (else
      (goto _label_5))))

(event `FacePlayer`
  (bind (_returnvalue_roll _returnvalue_pitch _returnvalue_yaw) (`KismetMathLibrary.BreakRotator` (`KismetMathLibrary.RInterpTo` (`self.K2_GetActorRotation`) (`KismetMathLibrary.FindLookAtRotation` (`self.K2_GetActorLocation`) (`self.K2_GetActorLocation` (`GameplayStatics.GetPlayerCharacter` 0))) (`GameplayStatics.GetWorldDeltaSeconds`) 1.5)))
  ;[0.001892 0 1 0.1] AI Sense
  ;;[0 0 1 0] Facing Constant Player if Player was seen
  (`self.K2_SetActorRotation` (`KismetMathLibrary.MakeRotator` 0.0 0.0 _returnvalue_yaw) :!label _label_6)
  (`KismetSystemLibrary.Delay` 0.001)
  (goto _label_6))

(event `self.Sphere.OnComponentBeginOverlap`
  (params (OverlappedComponent :type "PrimitiveComponent Object Reference") (OtherActor :type "Actor Object Reference") (OtherComp :type "PrimitiveComponent Object Reference") (OtherBodyIndex :type Integer) (bFromSweep :type Boolean) (SweepResult :type "HitResult Structure (by ref)"))
  ;[0.001892 0 1 0.1] AI Sense
  ;;[0 0 1 0] Turn to Player
  (bind _asbp_player_character_mert (cast `/Game/Devs/Mert/Blueprints/Player/BP_PlayerCharacterMert` OtherActor))
  (set `self.Player ref` _asbp_player_character_mert)
  (`self.FacePlayer`))

(event `self.StunSphereCollision.OnComponentBeginOverlap`
  (params (OverlappedComponent :type "PrimitiveComponent Object Reference") (OtherActor :type "Actor Object Reference") (OtherComp :type "PrimitiveComponent Object Reference") (OtherBodyIndex :type Integer) (bFromSweep :type Boolean) (SweepResult :type "HitResult Structure (by ref)"))
  (bind _mesh (`self.Mesh`))
  (bind _player_ref (`self.Player ref`))
  (bind _player_ref_2 (`self.Player ref`))
  ;[0.001892 0 1 0.1] AI Sense
  ;;[0 0 1 0] Stun Trigger
  (cast `/Game/Devs/Mert/Blueprints/Player/BP_PlayerCharacterMert` OtherActor)
  (`SceneComponent.SetHiddenInGame` (`self.SpotLight1`) true false)
  (`SceneComponent.SetRelativeScale3D` _mesh (0.0 0.0 0.0))
  (`SceneComponent.SetHiddenInGame` (`self.SkeletalMesh`) false false)
  (`SceneComponent.SetHiddenInGame` (`self.PointLight`) false false)
  (`/Engine/EditorBlueprintResources/StandardMacros.DoOnce` false
    (:`Completed`
      (bind (_direction _stun) (`Timeline|Timeline`)
        (:`Update`
          (bind _returnvalue (`KismetMathLibrary.Lerp` 0.0 (`self.Stun Value`) _stun))
          (`SceneComponent.SetRelativeScale3D` _mesh (`KismetMathLibrary.MakeVector` _returnvalue _returnvalue _returnvalue))
          (`/Engine/EditorBlueprintResources/StandardMacros.DoOnce` false
            (:`Completed`
              (`CharacterMovementComponent.DisableMovement` (`self.CharacterMovement`))
              (bind _returnvalue_2 (`AddComponent|NODE_AddAudioComponent-2` :`RelativeTransform` (`KismetMathLibrary.MakeTransform` (`self.K2_GetActorLocation`))))
              (set `self.RisingSound ref` _returnvalue_2))))
        (:`Finished`
          (set `self.EnemyHealth` 10.0)
          (bind _returnvalue_3 (`|CreateWidget` "/Game/Devs/Mert/Blueprints/Player/Widgets/W_Transitions/W_BlackBlend.W_BlackBlend_C"))
          (`UserWidget.AddToViewport` _returnvalue_3 0)
          (`/Game/Devs/Mert/Blueprints/Player/Widgets/W_Transitions/W_BlackBlend.ToBlackBlend` _returnvalue_3)
          (bind _returnvalue_4 (`|CreateWidget` "/Game/Devs/Mert/Blueprints/Player/Widgets/W_Feedback/W_Damage.W_Damage_C"))
          (`UserWidget.AddToViewport` _returnvalue_4 0)
          (`/Game/Devs/Mert/Blueprints/Player/Widgets/W_Feedback/W_Damage.DamageOpacity` _returnvalue_4)
          (if (> (`/Game/Devs/Mert/Blueprints/Player/BP_PlayerCharacterMert.PlayerHealth4` _player_ref) 0.0)
            (set `/Game/Devs/Mert/Blueprints/Player/BP_PlayerCharacterMert.PlayerHealth4` 0.0 _player_ref_2)
            (`KismetSystemLibrary.Delay` 1.0 :!label _label_7)
            (`self.K2_DestroyActor`)
            (`/Game/Devs/Mert/Blueprints/Player/Widgets/W_Transitions/W_BlackBlend.ToVisibleBlend` _returnvalue_3)
            (bind _outactors (`GameplayStatics.GetAllActorsOfClass` "/Game/Devs/Mert/Blueprints/Enemies/EnemyEntity1.EnemyEntity1_C"))
            (`/Game/Devs/Mert/Blueprints/Enemies/EnemyEntity1.FacePlayer` _outactors)
            (`/Game/Devs/Mert/Blueprints/Enemies/EnemyEntity1.MinionCalls` (`|GetArrayItem` _outactors))
            (`self.K2_DestroyActor`)
            (elif (> (`/Game/Devs/Mert/Blueprints/Player/BP_PlayerCharacterMert.PlayerHealth3` _player_ref) 0.0)
              (set `/Game/Devs/Mert/Blueprints/Player/BP_PlayerCharacterMert.PlayerHealth3` 0.0 _player_ref_2)
              (goto _label_7)
              (elif (> (`/Game/Devs/Mert/Blueprints/Player/BP_PlayerCharacterMert.PlayerHealth2` _player_ref) 0.0)
                (set `/Game/Devs/Mert/Blueprints/Player/BP_PlayerCharacterMert.PlayerHealth2` 0.0 _player_ref_2)
                (goto _label_7)
                (elif (> (`/Game/Devs/Mert/Blueprints/Player/BP_PlayerCharacterMert.PlayerHealth1` _player_ref) 0.0)
                  (set `/Game/Devs/Mert/Blueprints/Player/BP_PlayerCharacterMert.PlayerHealth1` 0.0 _player_ref_2)
                  (`/Game/Devs/Mert/Blueprints/Player/BP_PlayerCharacterMert.PlayerDeath` _player_ref_2))))))))))

(fn `UserConstructionScript`)