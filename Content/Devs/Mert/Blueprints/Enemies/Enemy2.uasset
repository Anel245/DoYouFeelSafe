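; Zombie enemy that roams, screams on spotting the player, chases and attacks, and destroys itself at zero health.
; Collapsed graphs drive it without a behavior tree: Tick runs random roaming, PawnSensing triggers chase through AIMoveTo.
; Timed attack flags gate DamageBox overlap damage, and failed moves clear sight after a delay.
; Sight, damage and sphere overlap start FacePlayer, an endless Delay loop interpolating yaw toward the player.
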(event `self.ReceiveTick`
  (params (DeltaSeconds :type "Float (single-precision)"))
  (`|ExecutionSequence`
    (:`then_0`
      (if (not (`self.IsMoving`))
        (`KismetSystemLibrary.Delay` (`KismetMathLibrary.RandomFloatInRange` 3.0 6.0))
        (if (not (`self.CanSeePlayer`))
          (`|ExecutionSequence`
            (:`then_0`
              (set `self.IsMoving` true)
              (`SkeletalMeshComponent.PlayAnimation` (`self.Mesh`) "/Game/Devs/Mert/Animations/Enemies/ZombieRun.ZombieRun" true)
              (set `CharacterMovementComponent.MaxWalkSpeed` 200.0 (`self.CharacterMovement`))
              (`|AIMoveTo` self (`NavigationSystemV1.K2_GetRandomReachablePointInRadius` (`self.K2_GetActorLocation`) 1500.0 null null) null 500.0
                (:`OnSuccess`
                  _)
                (:`OnFail`
                  _))
              (set `self.IsMoving` false)
              (`SkeletalMeshComponent.PlayAnimation` (`self.Mesh`) "/Game/Devs/Mert/Animations/Enemies/ZombieIdle.ZombieIdle" true))
            (:`then_1`
              (goto _label :!via `Reset`))))))))

(event `self.PawnSensing.OnSeePawn`
  (params (Pawn :type "Pawn Object Reference"))
  ;[1 1 1] See Player
  (cast `/Game/Devs/Mert/Blueprints/Player/BP_PlayerCharacterMert` Pawn)
  (set `self.CanSeePlayer` true)
  (`|ExecutionSequence`
    (:`then_0`
      (`/Engine/EditorBlueprintResources/StandardMacros.DoOnce` false :!label _label
        (:`Completed`
          (`MovementComponent.StopMovementImmediately` (`self.CharacterMovement`))
          (`self.FacePlayer`)
          (set `self.FirstSightScream` true)
          (`SkeletalMeshComponent.PlayAnimation` (`self.Mesh`) "/Game/Devs/Mert/Animations/Enemies/ZombieScream.ZombieScream" false)
          (`KismetSystemLibrary.Delay` 2.2)
          (set `self.FirstSightScream` false))))
    (:`then_1`
      (if (not (`self.FirstSightScream`))
        (`self.ChasePlayer`)
        (`self.FacePlayer`)))))

(event `ChasePlayer`
  ;[1 1 1] Following & Chasing Player
  (if (`self.CanSeePlayer`)
    (`|ExecutionSequence`
      (:`then_0`
        (`/Engine/EditorBlueprintResources/StandardMacros.DoOnce` false :!label _label_2
          (:`Completed`
            (`GameplayStatics.SpawnSound2D` "/Game/FPWeapon/Audio/FirstPersonTemplateWeaponFire02.FirstPersonTemplateWeaponFire02" 1.0 1.0 0.0 null)
            (`KismetSystemLibrary.PrintString` "I see you" true true (struct :`R` 1.0 :`G` 0.040784 :`A` 1.0)))))
      (:`then_1`
        (set `self.IsMoving` true)
        (set `CharacterMovementComponent.MaxWalkSpeed` 250.0 (`self.CharacterMovement`))
        (if (not (`self.AttackingPlayerAnimation`))
          (`|AIMoveTo` self (0.0 0.0 0.0) (`GameplayStatics.GetPlayerCharacter` 0) 200.0
            (:`OnSuccess`
              (set `self.CanSeePlayer` true)
              (set `self.IsMoving` true)
              (`/Engine/EditorBlueprintResources/StandardMacros.DoOnce` false :!label _label_3
                (:`Completed`
                  (`SkeletalMeshComponent.PlayAnimation` (`self.Mesh`) "/Game/Devs/Mert/Animations/Enemies/ZombieAttack.ZombieAttack" true)
                  (set `self.AttackingPlayerAnimation` true)
                  (`KismetSystemLibrary.Delay` 0.9)
                  (set `self.AttackingPlayer` true)
                  (`KismetSystemLibrary.Delay` 0.4)
                  (set `self.AttackingPlayer` false)
                  (`KismetSystemLibrary.Delay` 0.9)
                  (set `self.AttackingPlayerAnimation` false)
                  (`|ExecutionSequence`
                    (:`then_0`
                      (goto _label_3 :!via `Reset`))
                    (:`then_1`
                      (goto _label_6 :!via `Reset`))))))
            (:`OnFail`
              (`|ExecutionSequence`
                (:`then_0`
                  (`KismetSystemLibrary.Delay` 10.0 :!label _label_4)
                  (set `self.CanSeePlayer` false)
                  (set `self.IsMoving` false)
                  (`|ExecutionSequence`
                    (:`then_0`
                      (`/Engine/EditorBlueprintResources/StandardMacros.DoOnce` false :!label _label_5
                        (:`Completed`
                          (`GameplayStatics.SpawnSound2D` "/Game/Devs/Mert/Sounds/Flashlight_Switch.Flashlight_Switch" 1.0 1.0 0.0 null)
                          (`KismetSystemLibrary.PrintString` "Where did yu go?" true true (struct :`R` 1.0 :`G` 0.040784 :`A` 1.0))
                          (goto _label_2 :!via `Reset`))))
                    (:`then_1`
                      (goto _label_5 :!via `Reset`))))
                (:`then_1`
                  (if (not (`self.AttackingPlayerAnimation`))
                    (`/Engine/EditorBlueprintResources/StandardMacros.DoOnce` false :!label _label_6
                      (:`Completed`
                        (`SkeletalMeshComponent.PlayAnimation` (`self.Mesh`) "/Game/Devs/Mert/Animations/Enemies/ZombieRun.ZombieRun" true)))))))))))
    (else
      (goto _label_4))))

(event `self.Sphere.OnComponentBeginOverlap`
  (params (OverlappedComponent :type "PrimitiveComponent Object Reference") (OtherActor :type "Actor Object Reference") (OtherComp :type "PrimitiveComponent Object Reference") (OtherBodyIndex :type Integer) (bFromSweep :type Boolean) (SweepResult :type "HitResult Structure (by ref)"))
  ;[1 1 1] Turn around if Player is behind Enemy
  (bind _asbp_player_character_mert (cast `/Game/Devs/Mert/Blueprints/Player/BP_PlayerCharacterMert` OtherActor))
  (set `self.As BP Player Character Mert` _asbp_player_character_mert)
  (`self.FacePlayer`))

(event `FacePlayer`
  (bind (_returnvalue_roll _returnvalue_pitch _returnvalue_yaw) (`KismetMathLibrary.BreakRotator` (`KismetMathLibrary.RInterpTo` (`self.K2_GetActorRotation`) (`KismetMathLibrary.FindLookAtRotation` (`self.K2_GetActorLocation`) (`self.K2_GetActorLocation` (`GameplayStatics.GetPlayerCharacter` 0))) (`GameplayStatics.GetWorldDeltaSeconds`) 1.5)))
  ;[1 1 1] Facing Constant Player if Player was seen
  (`self.K2_SetActorRotation` (`KismetMathLibrary.MakeRotator` 0.0 0.0 _returnvalue_yaw) :!label _label_7)
  (`KismetSystemLibrary.Delay` 0.001)
  (goto _label_7))

(event `self.ReceiveAnyDamage`
  (params (Damage :type "Float (single-precision)") (DamageType :type "DamageType Object Reference") (InstigatedBy :type "Controller Object Reference") (DamageCauser :type "Actor Object Reference"))
  ;[1 1 1] Enemy Damaged
  (`self.FacePlayer`)
  (bind _output_get (set `self.EnemyHealth` (- (`self.EnemyHealth`) Damage)))
  (if (<= _output_get 0.0)
    (`self.K2_DestroyActor`)))

(event `self.DamageBox.OnComponentBeginOverlap`
  (params (OverlappedComponent :type "PrimitiveComponent Object Reference") (OtherActor :type "Actor Object Reference") (OtherComp :type "PrimitiveComponent Object Reference") (OtherBodyIndex :type Integer) (bFromSweep :type Boolean) (SweepResult :type "HitResult Structure (by ref)"))
  ;[1 1 1] Damage Player
  (bind _asbp_player_character_mert (cast `/Game/Devs/Mert/Blueprints/Player/BP_PlayerCharacterMert` OtherActor))
  (if (`self.AttackingPlayer`)
    (set `/Game/Devs/Mert/Blueprints/Player/BP_PlayerCharacterMert.PlayerDamage` true _asbp_player_character_mert)
    (`/Game/Devs/Mert/Blueprints/Player/BP_PlayerCharacterMert.Damage50%` _asbp_player_character_mert)
    (set `/Game/Devs/Mert/Blueprints/Player/BP_PlayerCharacterMert.PlayerDamage` false _asbp_player_character_mert)))

(fn `UserConstructionScript`)