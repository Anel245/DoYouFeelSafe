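; Hiding-spot pawn the player possesses through Interact and leaves by possessing BP_PlayerCharacterMert again, with black fade and creak sound.
; Its cube meshes show only while possessed.
; While active, a delayed Tick copies health, stamina and inventory one-way from the character and runs stamina recovery on the local copy.
; Collapsed graphs handle medicine, batteries, inventory HUD, pause menu and line-trace autofocus depth of field.
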(event `self.ReceiveTick`
  (params (DeltaSeconds :type "Float (single-precision)"))
  ;[1 0 0] EventTick
  (`KismetSystemLibrary.Delay` 0.2)
  (if (`self.PlayerHidActive`)
    (`|ExecutionSequence`
      (:`then_0`
        (set `self.HealingHid` false)
        (bind _asbp_player_character_mert (cast `/Game/Devs/Mert/Blueprints/Player/BP_PlayerCharacterMert` (`GameplayStatics.GetPlayerCharacter` 0)))
        (set `self.PlayerHealth1Hid` (`/Game/Devs/Mert/Blueprints/Player/BP_PlayerCharacterMert.PlayerHealth1` _asbp_player_character_mert))
        (set `self.PlayerHealth2Hid` (`/Game/Devs/Mert/Blueprints/Player/BP_PlayerCharacterMert.PlayerHealth2` _asbp_player_character_mert))
        (set `self.PlayerHealth3Hid` (`/Game/Devs/Mert/Blueprints/Player/BP_PlayerCharacterMert.PlayerHealth3` _asbp_player_character_mert))
        (set `self.PlayerHealth4Hid` (`/Game/Devs/Mert/Blueprints/Player/BP_PlayerCharacterMert.PlayerHealth4` _asbp_player_character_mert))
        (set `self.PlayerStaminaHid` (`/Game/Devs/Mert/Blueprints/Player/BP_PlayerCharacterMert.PlayerStamina` _asbp_player_character_mert))
        (set `self.FlashlightBatteryHid` (`/Game/Devs/Mert/Blueprints/Player/BP_PlayerCharacterMert.FlashlightBattery` _asbp_player_character_mert))
        (set `self.HasWeaponHid` (`/Game/Devs/Mert/Blueprints/Player/BP_PlayerCharacterMert.HasWeapon` _asbp_player_character_mert))
        (set `self.HasFlashlightHid` (`/Game/Devs/Mert/Blueprints/Player/BP_PlayerCharacterMert.HasFlashlight` _asbp_player_character_mert))
        (set `self.HasKeyHid` (`/Game/Devs/Mert/Blueprints/Player/BP_PlayerCharacterMert.HasKey` _asbp_player_character_mert))
        (set `self.HasHandleHid` (`/Game/Devs/Mert/Blueprints/Player/BP_PlayerCharacterMert.HasHandle` _asbp_player_character_mert))
        (set `self.HasSpecialItemHid` (`/Game/Devs/Mert/Blueprints/Player/BP_PlayerCharacterMert.HasSpecialItem` _asbp_player_character_mert))
        (set `self.MedicineCountHid` (`/Game/Devs/Mert/Blueprints/Player/BP_PlayerCharacterMert.MedicineCount` _asbp_player_character_mert))
        (set `self.BatteryCountHid` (`/Game/Devs/Mert/Blueprints/Player/BP_PlayerCharacterMert.BatteryCount` _asbp_player_character_mert))
        (set `self.PistolAmmoHid` (`/Game/Devs/Mert/Blueprints/Player/BP_PlayerCharacterMert.PistolAmmo` _asbp_player_character_mert))
        (set `self.PistolMaxAmmoHid` (`/Game/Devs/Mert/Blueprints/Player/BP_PlayerCharacterMert.PistolMaxAmmo` _asbp_player_character_mert))
        (set `/Game/Devs/Mert/Blueprints/Player/BP_PlayerCharacterMert.CameraCount` (`/Game/Devs/Mert/Blueprints/Player/BP_PlayerCharacterMert.CameraCount` _asbp_player_character_mert) _asbp_player_character_mert))
      (:`then_1`
        (if (< (`self.PlayerStaminaHid`) 1.0)
          (`KismetSystemLibrary.Delay` 4.0 :!label _label)
          (if (< (`self.PlayerStaminaHid`) 1.0) :!label _label_2
            (`KismetSystemLibrary.Delay` 0.002)
            (set `self.PlayerStaminaHid` (+ (`self.PlayerStaminaHid`) 0.004))
            (goto _label_2)
            (else
              (goto _label))))))))

(event `/Game/Devs/Mert/Blueprints/Player/Interfaces/InteractionInterface.Interact`
  ;[1 1 1] Possessed
  (bind _returnvalue (`|CreateWidget` "/Game/Devs/Mert/Blueprints/Player/Widgets/W_Transitions/W_BlackBlend.W_BlackBlend_C"))
  (`UserWidget.AddToViewport` _returnvalue 0)
  (`/Game/Devs/Mert/Blueprints/Player/Widgets/W_Transitions/W_BlackBlend.BlackTransition` _returnvalue)
  (`GameplayStatics.PlaySoundAtLocation` "/Game/Devs/Mert/Sounds/Environment/WoodFloorCreak.WoodFloorCreak" (`self.K2_GetActorLocation`) (struct) 0.8 (`KismetMathLibrary.RandomFloatInRange` 0.95 1.15) 0.0 null null null null)
  (`KismetSystemLibrary.Delay` 1.5)
  (`Controller.Possess` (`GameplayStatics.GetPlayerController` 0) self)
  (set `self.PlayerHidActive` true))

(event `self.ReceiveBeginPlay`
  ;[1 1 1] Visibility
  (`SceneComponent.SetHiddenInGame` (`self.Cube1`) true false)
  (`SceneComponent.SetHiddenInGame` (`self.Cube2`) true false)
  (`SceneComponent.SetHiddenInGame` (`self.Cube3`) true false)
  (`SceneComponent.SetHiddenInGame` (`self.Cube4`) true false)
  (`SceneComponent.SetHiddenInGame` (`self.Cube5`) true false)
  (`SceneComponent.SetHiddenInGame` (`self.Cube6`) true false)
  (`SceneComponent.SetHiddenInGame` (`self.Cube`) true false))

(event `InputAction|Interact`
  (params (Key :type "Key Structure"))
  ;[1 1 1] Unpossessed
  (:`Pressed`
    (bind _returnvalue (`|CreateWidget` "/Game/Devs/Mert/Blueprints/Player/Widgets/W_Transitions/W_BlackBlend.W_BlackBlend_C"))
    (`UserWidget.AddToViewport` _returnvalue 0)
    (`/Game/Devs/Mert/Blueprints/Player/Widgets/W_Transitions/W_BlackBlend.BlackTransition` _returnvalue)
    (`GameplayStatics.PlaySoundAtLocation` "/Game/Devs/Mert/Sounds/Environment/WoodFloorCreak.WoodFloorCreak" (`self.K2_GetActorLocation`) (struct) 0.8 (`KismetMathLibrary.RandomFloatInRange` 0.8 0.95) 0.0 null null null null)
    (`KismetSystemLibrary.Delay` 1.5)
    (bind _outactors (`GameplayStatics.GetAllActorsOfClass` "/Game/Devs/Mert/Blueprints/Player/BP_PlayerCharacterMert.BP_PlayerCharacterMert_C"))
    (`Controller.Possess` (`GameplayStatics.GetPlayerController` 0) (`|GetArrayItem` _outactors))
    (set `self.PlayerHidActive` false)
    (if (`self.IsInventoryActiveHid`)
      (set `self.IsInventoryActiveHid` false)
      (`Widget.RemoveFromParent` (`self.PlayerInfoHUDrefHid`)))))

(event `self.ReceivePossessed`
  (params (NewController :type "Controller Object Reference"))
  ;[1 1 1] Visibility
  (`SceneComponent.SetHiddenInGame` (`self.Cube6`) false false)
  (`SceneComponent.SetHiddenInGame` (`self.Cube5`) false false)
  (`SceneComponent.SetHiddenInGame` (`self.Cube4`) false false)
  (`SceneComponent.SetHiddenInGame` (`self.Cube3`) false false)
  (`SceneComponent.SetHiddenInGame` (`self.Cube2`) false false)
  (`SceneComponent.SetHiddenInGame` (`self.Cube1`) false false)
  (`SceneComponent.SetHiddenInGame` (`self.Cube`) false false))

(event `InputAction|PauseMenu` :paused true
  (params (Key :type "Key Structure"))
  (bind _returnvalue (`GameplayStatics.GetPlayerController` 0))
  ;[1 1 1] Pause
  (:`Pressed`
    (if (`GameplayStatics.IsGamePaused`)
      (`Widget.RemoveFromParent` (stale _returnvalue_2))
      (`GameplayStatics.SetGamePaused` false)
      (set `PlayerController.bShowMouseCursor` false _returnvalue)
      (`WidgetBlueprintLibrary.SetInputMode_GameOnly` _returnvalue)
      (set `self.IsGameActiveHid` true)
      (else
        (bind _returnvalue_2 (`|CreateWidget` "/Game/Devs/Mert/Blueprints/Player/Widgets/W_Options/W_MenuPause.W_MenuPause_C"))
        (bind _output_get (set `self.PauseHUDrefHid` _returnvalue_2))
        (`UserWidget.AddToViewport` _output_get 0)
        (`GameplayStatics.SetGamePaused` true)
        (set `PlayerController.bShowMouseCursor` true _returnvalue)
        (`WidgetBlueprintLibrary.SetInputMode_GameAndUIEx` _returnvalue _returnvalue_2 "LockInFullscreen")
        (set `self.IsGameActiveHid` false)
        (bind _returnvalue_3 (`|CreateWidget` "/Game/Devs/Mert/Blueprints/Player/Widgets/W_Options/W_MenuOptions.W_MenuOptions_C"))
        (bind _output_get_2 (set `self.OptionsHUDrefHid` _returnvalue_3))
        (`/Game/Devs/Mert/Blueprints/Player/Widgets/W_Options/W_MenuOptions.Load Settings` _output_get_2)))))

(event `InputAction|Medicine Usage`
  (params (Key :type "Key Structure"))
  (bind _medicinecounthid (`self.MedicineCountHid`))
  ;[1 1 1] Medicine Usage
  (:`Pressed`
    (if (> _medicinecounthid 0)
      (if (< (`self.PlayerHealth1Hid`) 1.0)
        (set `self.HealingHid` true)
        (set `self.PlayerHealth1Hid` 1.0)
        (set `self.MedicineCountHid` (- _medicinecounthid 1) :!label _label_3)
        (bind _returnvalue (`|CreateWidget` "/Game/Devs/Mert/Blueprints/Player/Widgets/W_Feedback/W_Health.W_Health_C"))
        (`UserWidget.AddToViewport` _returnvalue 0)
        (elif (< (`self.PlayerHealth2Hid`) 1.0)
          (set `self.HealingHid` true)
          (set `self.PlayerHealth2Hid` 1.0)
          (goto _label_3)
          (elif (< (`self.PlayerHealth3Hid`) 1.0)
            (set `self.HealingHid` true)
            (set `self.PlayerHealth3Hid` 1.0)
            (goto _label_3)
            (elif (< (`self.PlayerHealth4Hid`) 1.0)
              (set `self.HealingHid` true)
              (set `self.PlayerHealth4Hid` 1.0)
              (goto _label_3)
              (else
                (`KismetSystemLibrary.PrintString` "You are not hurt!"))))))
      (else
        (`KismetSystemLibrary.PrintString` "You dont have any Medicine!")))))

(event `self.ReceiveUnpossessed`
  (params (OldController :type "Controller Object Reference"))
  ;[1 1 1] Visibility
  (`SceneComponent.SetHiddenInGame` (`self.Cube1`) true false)
  (`SceneComponent.SetHiddenInGame` (`self.Cube3`) true false)
  (`SceneComponent.SetHiddenInGame` (`self.Cube4`) true false)
  (`SceneComponent.SetHiddenInGame` (`self.Cube5`) true false)
  (`SceneComponent.SetHiddenInGame` (`self.Cube6`) true false)
  (`SceneComponent.SetHiddenInGame` (`self.Cube2`) true false)
  (`SceneComponent.SetHiddenInGame` (`self.Cube`) true false))

(event `InputAction|Inventory & Info`
  (params (Key :type "Key Structure"))
  (bind _playerinfohudrefhid (`self.PlayerInfoHUDrefHid`))
  ;[1 1 1] Info & Inventory HUD
  (:`Pressed`
    (if (`self.IsInventoryActiveHid`)
      (set `self.IsInventoryActiveHid` false)
      (`/Game/Devs/Mert/Blueprints/Player/Widgets/W_Feedback/W_PlayerInfoHUD.InventoryFadeOut` _playerinfohudrefhid)
      (else
        (set `self.IsInventoryActiveHid` true)
        (bind _returnvalue (`|CreateWidget` "/Game/Devs/Mert/Blueprints/Player/Widgets/W_Feedback/W_PlayerInfoHUD.W_PlayerInfoHUD_C"))
        (bind _output_get (set `self.PlayerInfoHUDrefHid` _returnvalue))
        (`UserWidget.AddToViewport` _output_get 0)
        (`/Game/Devs/Mert/Blueprints/Player/Widgets/W_Feedback/W_PlayerInfoHUD.InventoryFadeIn` _playerinfohudrefhid)))))

(event `InputAction|Battery Usage`
  (params (Key :type "Key Structure"))
  ;[1 1 1] Battery Usage
  (:`Pressed`
    (if (`self.HasFlashlightHid`)
      (if (> (`self.BatteryCountHid`) 0)
        (set `self.FlashlightBatteryHid` 1.0)
        (set `self.BatteryCountHid` (- (`self.BatteryCountHid`) 1))
        (bind _returnvalue (`|CreateWidget` "/Game/Devs/Mert/Blueprints/Player/Widgets/W_Feedback/W_Flash.W_Flash_C"))
        (`UserWidget.AddToViewport` _returnvalue 0)
        (else
          (`KismetSystemLibrary.PrintString` "You don't have any Batteries!")))
      (else
        (`KismetSystemLibrary.PrintString` "You need an Flashlight to use Batteries!")))))

(event `DepthOfField`
  (bind _camera (`self.Camera`))
  (bind _camera_2 (`self.Camera`))
  (bind _returnvalue (`SceneComponent.K2_GetComponentLocation` _camera_2))
  (bind (_outhit _returnvalue_2) (`KismetSystemLibrary.LineTraceSingle` _returnvalue (+ _returnvalue (* (`KismetMathLibrary.GetForwardVector` (`SceneComponent.K2_GetComponentRotation` _camera_2)) (`KismetMathLibrary.Conv_DoubleToVector` 5000.0))) "TraceTypeQuery2"))
  (if _returnvalue_2
    (bind _output_get (set `self.FocusedLocation` (`KismetMathLibrary.VSize` (- (`.Location` (`GameplayStatics.BreakHitResult` _outhit)) (`SceneComponent.K2_GetComponentLocation` _camera)))))
    (set `CameraComponent.PostProcessSettings` (make `PostProcessSettings` :`DepthOfFieldFstop` 0.5 :`DepthOfFieldMinFstop` 11.0 :`DepthOfFieldFocalDistance` _output_get) _camera)))

(fn `UserConstructionScript`)