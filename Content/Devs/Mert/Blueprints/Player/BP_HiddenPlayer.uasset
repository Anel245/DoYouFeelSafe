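; BP_HiddenPlayer is an interactable hiding spot that the player can enter and leave.
; Interact, gated by the player's 1Loop flag, disables collision, blends the view to this actor and plays a door timeline rotating three meshes.
; After a delay it hides the player and ignores look input, then polls the F key on a Delay loop.
; Pressing F reverses the door, restores the player and view, and calls PlayerTurnAround.
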(event `/Game/Devs/Mert/Blueprints/Player/Interfaces/InteractionInterface.Interact`
  (bind _returnvalue (`GameplayStatics.GetPlayerController` 0))
  (bind _playermertref (`self.PlayerMertref`))
  (bind _playermertref_2 (`self.PlayerMertref`))
  (bind _playermertref_3 (`self.PlayerMertref`))
  (bind _asbp_player_character_mert_new (cast `/Game/Devs/Mert/Blueprints/Player/BP_PlayerCharacterMertNew` (`GameplayStatics.GetPlayerCharacter` 0)))
  (bind _output_get (set `self.PlayerMertref` _asbp_player_character_mert_new))
  (if (not (`/Game/Devs/Mert/Blueprints/Player/BP_PlayerCharacterMertNew.1 Loop` _output_get))
    (set `/Game/Devs/Mert/Blueprints/Player/BP_PlayerCharacterMertNew.Interacting` true _output_get)
    (if (not (`self.Hiding`))
      (`GameplayStatics.PlaySoundAtLocation` "/Game/Devs/Mert/Sounds/Environment/WoodFloorCreak.WoodFloorCreak" (`self.K2_GetActorLocation`) (struct) 0.8 (`KismetMathLibrary.RandomFloatInRange` 0.95 1.15) 0.0 null null null null)
      (set `self.Hiding` true)
      (`self.SetActorEnableCollision` _playermertref false)
      (set `/Game/Devs/Mert/Blueprints/Player/BP_PlayerCharacterMertNew.IsPlayerActive` false _playermertref)
      (`PlayerController.SetViewTargetWithBlend` (`GameplayStatics.GetPlayerController` 0) self 1.2 "VTBlend_Linear" 1.2 false) ; Possess
      (`|ExecutionSequence`
        (:`then_0`
          (bind (_direction _door) (`Timeline|OpenCloseDoorTL` :!label _label)
            (:`Update`
              (`SceneComponent.K2_SetRelativeRotation` (`self.Sphere5`) (`KismetMathLibrary.MakeRotator` 180.0 0.0 (`KismetMathLibrary.Lerp` (`self.CloseAngle`) (`self.OpenAngle`) _door)) false false)
              (`SceneComponent.K2_SetRelativeRotation` (`self.Sphere12`) (`KismetMathLibrary.MakeRotator` 180.0 0.0 (`KismetMathLibrary.Lerp` (`self.CloseAngle`) (`self.OpenAngle`) _door)) false false)
              (`SceneComponent.K2_SetRelativeRotation` (`self.Sphere14`) (`KismetMathLibrary.MakeRotator` 180.0 0.0 (`KismetMathLibrary.Lerp` (`self.CloseAngle`) (`self.OpenAngle`) _door)) false false))))
        (:`then_1`
          (`KismetSystemLibrary.Delay` 1.0)
          (`self.SetActorHiddenInGame` (`self.PlayerMertref`) true)
          (`Controller.SetIgnoreLookInput` _returnvalue true)
          (if (`PlayerController.IsInputKeyDown` _returnvalue "F") :!label _label_2
            (`GameplayStatics.PlaySoundAtLocation` "/Game/Devs/Mert/Sounds/Environment/WoodFloorCreak.WoodFloorCreak" (`self.K2_GetActorLocation`) (struct) 0.8 (`KismetMathLibrary.RandomFloatInRange` 0.8 0.95) 0.0 null null null null)
            (set `self.Hiding` false)
            (`self.SetActorEnableCollision` _playermertref_2 true)
            (`PlayerController.SetViewTargetWithBlend` (`GameplayStatics.GetPlayerController` 0) _playermertref_2 1.0 "VTBlend_Linear" 0.0 false) ; Unpossess
            (`/Game/Devs/Mert/Blueprints/Player/BP_PlayerCharacterMertNew.PlayerTurnAround` _playermertref_2)
            (`|ExecutionSequence`
              (:`then_0`
                (`KismetSystemLibrary.Delay` 1.0)
                (`self.SetActorHiddenInGame` _playermertref_3 false)
                (set `/Game/Devs/Mert/Blueprints/Player/BP_PlayerCharacterMertNew.IsPlayerActive` true _playermertref_3)
                (`Controller.ResetIgnoreLookInput` _returnvalue))
              (:`then_1`
                (goto _label :!via `Reverse`)))
            (else
              (`KismetSystemLibrary.Delay` 0.2)
              (goto _label_2))))))))

(fn `UserConstructionScript`)