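; Pistol pickup actor that arms the player when interacted with.
; Interact casts the player character to BP_PlayerCharacterMert, sets HasWeapon, plays the pickup sound at its location and destroys itself.
; As player feedback, Tick runs a chain of Delays that periodically double-flashes a point light, relying on latent delays ignoring re-triggers instead of using a timer.
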(event `self.ReceiveTick`
  (params (DeltaSeconds :type "Float (single-precision)"))
  ;[1 1 1] PlayerFeedback
  (`KismetSystemLibrary.Delay` 7.5)
  (`SceneComponent.SetHiddenInGame` (`self.PointLight`) false false)
  (`KismetSystemLibrary.Delay` 0.1)
  (`SceneComponent.SetHiddenInGame` (`self.PointLight`) true false)
  (`KismetSystemLibrary.Delay` 0.1)
  (`SceneComponent.SetHiddenInGame` (`self.PointLight`) false false)
  (`KismetSystemLibrary.Delay` 0.1)
  (`SceneComponent.SetHiddenInGame` (`self.PointLight`) true false))

(event `/Game/Devs/Mert/Blueprints/Player/Interfaces/InteractionInterface.Interact`
  ;[1 1 1] Interact
  (bind _asbp_player_character_mert (cast `/Game/Devs/Mert/Blueprints/Player/BP_PlayerCharacterMert` (`GameplayStatics.GetPlayerCharacter` 0)))
  (set `/Game/Devs/Mert/Blueprints/Player/BP_PlayerCharacterMert.HasWeapon` true _asbp_player_character_mert)
  (`GameplayStatics.PlaySoundAtLocation` "/Game/Devs/Mert/Sounds/PickUp.PickUp" (`self.K2_GetActorLocation`) (struct) 1.0 1.0 0.0 null null null null)
  (`self.K2_DestroyActor`))

(fn `UserConstructionScript`)