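; Medicine pickup actor that adds to the MedicineCount of BP_PlayerCharacterMert when interacted with, up to a carry limit of five.
; Interact checks the count through nested branches, then either increments it, spawns an emitter and sound and destroys the actor, or prints a full-inventory message.
; Tick runs a chain of Delays that periodically double-blinks the PointLight as player feedback.
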(event `self.ReceiveBeginPlay`)

(event `self.ReceiveTick`
  (params (DeltaSeconds :type "Float (single-precision)"))
  ;[1 1 1] PlayerFeedback
  (`KismetSystemLibrary.Delay` 7.5)
  (`SceneComponent.SetHiddenInGame` (`self.PointLight`) false false)
  (`KismetSystemLibrary.Delay` 0.1)
  (`SceneComponent.SetHiddenInGame` (`self.PointLight`) true false)
  (`KismetSystemLibrary.Delay` 0.1)
  (`SceneComponent.SetHiddenInGame` (`self.PointLight`) false false)
  (`KismetSystemLibrary.Delay` 0.1)
  (`SceneComponent.SetHiddenInGame` (`self.PointLight`) true false))

(event `/Game/Devs/Mert/Blueprints/Player/Interfaces/InteractionInterface.Interact`
  (bind _returnvalue (`self.K2_GetActorLocation`))
  ;[1 1 1] Interaction
  (bind _asbp_player_character_mert (cast `/Game/Devs/Mert/Blueprints/Player/BP_PlayerCharacterMert` (`GameplayStatics.GetPlayerCharacter` 0)))
  (bind _medicinecount (`/Game/Devs/Mert/Blueprints/Player/BP_PlayerCharacterMert.MedicineCount` _asbp_player_character_mert))
  (if (== _medicinecount 0)
    (set `/Game/Devs/Mert/Blueprints/Player/BP_PlayerCharacterMert.MedicineCount` (+ _medicinecount 1) _asbp_player_character_mert :!label _label)
    (`GameplayStatics.SpawnEmitterAtLocation` null _returnvalue (struct :`Pitch` 90.0) (0.5 0.5 0.5))
    (`GameplayStatics.SpawnSoundAtLocation` "/Game/Devs/Mert/Sounds/PickUpSound.PickUpSound" _returnvalue (struct) 1.0 1.0 0.0 null null)
    (`KismetSystemLibrary.PrintString` "Picked Up Medicine" true true (struct :`G` 1.0 :`B` 0.991838 :`A` 1.0) 3.0)
    (`self.K2_DestroyActor`)
    (elif (== _medicinecount 1)
      (goto _label)
      (elif (== _medicinecount 2)
        (goto _label)
        (elif (== _medicinecount 3)
          (goto _label)
          (elif (== _medicinecount 4)
            (goto _label)
            (elif (== _medicinecount 5)
              (`KismetSystemLibrary.PrintString` "You can not carry any more!"))))))))

(fn `UserConstructionScript`)