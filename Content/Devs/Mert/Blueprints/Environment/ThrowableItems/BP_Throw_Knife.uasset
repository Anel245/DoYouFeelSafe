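; Throwable knife pickup that the player can collect and that can later be launched as a physics object.
; Interacting sets the player's HasKnife flag with particle and sound feedback, or shows a can't-pick-up widget if already holding a knife, fork or plate.
; KnifeThrow activates projectile movement and physics, pushing the knife away from the player's location.
; Impacts play a sound, rate-limited by a briefly reset DoOnce.
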(event `self.ReceiveBeginPlay`
  (`ActorComponent.SetActive` (`self.ProjectileMovement`) false false))

(event `KnifeThrow`
  ;[1 1 1] Throwable
  (`ActorComponent.SetActive` (`self.ProjectileMovement`) true false)
  (`PrimitiveComponent.SetSimulatePhysics` (`self.Item`) true)
  (bind _asbp_player_character_mert (cast `/Game/Devs/Mert/Blueprints/Player/BP_PlayerCharacterMert` (`GameplayStatics.GetPlayerCharacter` 0)))
  (`PrimitiveComponent.SetPhysicsLinearVelocity` (`self.Item`) (* (`KismetMathLibrary.GetDirectionUnitVector` (`self.K2_GetActorLocation` _asbp_player_character_mert) (`self.K2_GetActorLocation`)) 1000.0) false "None"))

(event `/Game/Devs/Mert/Blueprints/Player/Interfaces/InteractionInterface.Interact`
  (bind _returnvalue (`self.K2_GetActorLocation`))
  ;[1 1 1] Interaction
  (bind _asbp_player_character_mert (cast `/Game/Devs/Mert/Blueprints/Player/BP_PlayerCharacterMert` (`GameplayStatics.GetPlayerCharacter` 0)))
  (if (or (`/Game/Devs/Mert/Blueprints/Player/BP_PlayerCharacterMert.HasKnife` _asbp_player_character_mert) (`/Game/Devs/Mert/Blueprints/Player/BP_PlayerCharacterMert.HasFork` _asbp_player_character_mert) (`/Game/Devs/Mert/Blueprints/Player/BP_PlayerCharacterMert.HasPlate` _asbp_player_character_mert))
    (bind _returnvalue_2 (`|CreateWidget` "/Game/Devs/Mert/Blueprints/Player/Widgets/W_Dialogue/W_CantPickUp.W_CantPickUp_C"))
    (`UserWidget.AddToViewport` _returnvalue_2 0)
    (`/Game/Devs/Mert/Blueprints/Player/Widgets/W_Dialogue/W_CantPickUp.Opacity` _returnvalue_2)
    (else
      (set `/Game/Devs/Mert/Blueprints/Player/BP_PlayerCharacterMert.HasKnife` true _asbp_player_character_mert)
      (`GameplayStatics.SpawnEmitterAtLocation` null _returnvalue (struct :`Pitch` 90.0) (0.5 0.5 0.5))
      (`GameplayStatics.SpawnSoundAtLocation` "/Game/Devs/Mert/Sounds/PickUp.PickUp" _returnvalue (struct) 1.0 1.0 0.0 null null)
      (`self.K2_DestroyActor`))))

(event `self.ReceiveHit`
  (params (MyComp :type "PrimitiveComponent Object Reference") (Other :type "Actor Object Reference") (OtherComp :type "PrimitiveComponent Object Reference") (bSelfMoved :type Boolean) (HitLocation :type "Vector Structure") (HitNormal :type "Vector Structure") (NormalImpulse :type "Vector Structure") (Hit :type "HitResult Structure (by ref)"))
  ;[1 1 1] Hit Sound
  (`|ExecutionSequence`
    (:`then_0`
      (`/Engine/EditorBlueprintResources/StandardMacros.DoOnce` false :!label _label
        (:`Completed`
          (`GameplayStatics.PlaySoundAtLocation` "/Game/Devs/Mert/Sounds/PickUp.PickUp" HitLocation (struct) 0.8 1.2 0.0 null null null null))))
    (:`then_1`
      (`KismetSystemLibrary.Delay` 0.01)
      (goto _label :!via `Reset`))))

(fn `UserConstructionScript`)