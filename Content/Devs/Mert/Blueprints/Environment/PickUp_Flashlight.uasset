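; Flashlight pickup that grants the player a flashlight when touched.
; On Box overlap with BP_PlayerCharacterMert it sets HasFlashlight, spawns an emitter and a pickup sound at its location, then destroys itself.
; As player feedback, Tick runs a chain of delays that periodically double-blinks the PointLight to draw attention to the item.
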(event `self.ReceiveBeginPlay`)

(event `self.ReceiveTick`
  (params (DeltaSeconds :type "Float (single-precision)"))
  ;[1 1 1] PlayerFeedback
  (`KismetSystemLibrary.Delay` 7.5)
  (`SceneComponent.SetHiddenInGame` (`self.PointLight`) false false)
  (`KismetSystemLibrary.Delay` 0.1)
  (`SceneComponent.SetHiddenInGame` (`self.PointLight`) true false)
  (`KismetSystemLibrary.Delay` 0.1)
  (`SceneComponent.SetHiddenInGame` (`self.PointLight`) false false)
  (`KismetSystemLibrary.Delay` 0.1)
  (`SceneComponent.SetHiddenInGame` (`self.PointLight`) true false))

(event `self.Box.OnComponentBeginOverlap`
  (params (OverlappedComponent :type "PrimitiveComponent Object Reference") (OtherActor :type "Actor Object Reference") (OtherComp :type "PrimitiveComponent Object Reference") (OtherBodyIndex :type Integer) (bFromSweep :type Boolean) (SweepResult :type "HitResult Structure (by ref)"))
  (bind _returnvalue (`self.K2_GetActorLocation`))
  ;[1 1 1] Interaction
  (bind _asbp_player_character_mert (cast `/Game/Devs/Mert/Blueprints/Player/BP_PlayerCharacterMert` OtherActor))
  (set `/Game/Devs/Mert/Blueprints/Player/BP_PlayerCharacterMert.HasFlashlight` true _asbp_player_character_mert)
  (`GameplayStatics.SpawnEmitterAtLocation` null _returnvalue (struct :`Pitch` 90.0) (0.5 0.5 0.5))
  (`GameplayStatics.SpawnSoundAtLocation` "/Game/Devs/Mert/Sounds/PickUpSound.PickUpSound" _returnvalue (struct) 1.0 1.0 0.0 null null)
  (`self.K2_DestroyActor`))

(fn `UserConstructionScript`)