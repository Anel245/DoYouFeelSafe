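; Pickup actor that grants the tactical light ("TecLight") to the player's handgun character.
; On interact it casts the player to BP_LPSP_CH_Handgun, sets HasTecLight, spawns an effect and sound, prints a message and destroys itself.
; As player feedback, a chain of Delays on Tick periodically double-blinks its point light about every eight seconds.
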(event `self.ReceiveBeginPlay`)

(event `self.ReceiveTick`
  (params (DeltaSeconds :type "Float (single-precision)"))
  ;[1 1 1] PlayerFeedback
  (`KismetSystemLibrary.Delay` 7.5)
  (`SceneComponent.SetHiddenInGame` (`self.PointLight`) false false)
  (`KismetSystemLibrary.Delay` 0.1)
  (`SceneComponent.SetHiddenInGame` (`self.PointLight`) true false)
  (`KismetSystemLibrary.Delay` 0.1)
  (`SceneComponent.SetHiddenInGame` (`self.PointLight`) false false)
  (`KismetSystemLibrary.Delay` 0.1)
  (`SceneComponent.SetHiddenInGame` (`self.PointLight`) true false))

(event `/Game/Blueprints/Interfaces/InteractionInterface.Interact`
  (bind _returnvalue (`self.K2_GetActorLocation`))
  ;[1 1 1] Interaction
  (bind _asbp_lpsp_ch_handgun (cast `/LPSPSample/LPSPSample/Useable/Characters/BP_LPSP_CH_Handgun` (`GameplayStatics.GetPlayerCharacter` 0)))
  (set `/LPSPSample/LPSPSample/Useable/Characters/BP_LPSP_CH_Handgun.HasTecLight` true _asbp_lpsp_ch_handgun)
  (`GameplayStatics.SpawnEmitterAtLocation` "/Game/MilitaryWeapDark/FX/P_SniperRifle_MuzzleFlash_01.P_SniperRifle_MuzzleFlash_01" _returnvalue (struct :`Pitch` 90.0) (0.5 0.5 0.5))
  (`GameplayStatics.SpawnSoundAtLocation` "/Game/MilitaryWeapDark/Sound/Rifle/Wavs/Rifle_Reload03.Rifle_Reload03" _returnvalue (struct) 1.0 1.0 0.0 null null)
  (`self.K2_DestroyActor`)
  (`KismetSystemLibrary.PrintString` "Picked Up TecLight" true true (struct :`G` 1.0 :`B` 0.991838 :`A` 1.0) 3.0))

(fn `UserConstructionScript`)