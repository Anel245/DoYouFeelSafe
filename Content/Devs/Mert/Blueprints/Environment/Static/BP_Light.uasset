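; BP_Light is an environment light that reacts to the player's loop progress and to enemy sight.
; Tick passes through a one-second Delay, then reads loop flags on BP_PlayerCharacterMertNew to toggle PointLight1 and PointLight2 visibility; the third loop branch is empty.
; It also checks the first EnemyEntity1 found, applying a flicker light function material to PointLight2 while that enemy can see the player, clearing it otherwise.
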(event `self.ReceiveTick`
  (params (DeltaSeconds :type "Float (single-precision)"))
  (bind _pointlight2 (`self.PointLight2`))
  (`KismetSystemLibrary.Delay` 1.0)
  (bind _asbp_player_character_mert_new (cast `/Game/Devs/Mert/Blueprints/Player/BP_PlayerCharacterMertNew` (`GameplayStatics.GetPlayerPawn` 0)))
  (bind _outactors (`GameplayStatics.GetAllActorsOfClass` "/Game/Devs/Mert/Blueprints/Enemies/EnemyEntity1.EnemyEntity1_C"))
  (`|ExecutionSequence`
    (:`then_0`
      (if (`/Game/Devs/Mert/Blueprints/Player/BP_PlayerCharacterMertNew.1 Loop` _asbp_player_character_mert_new)
        (`SceneComponent.SetHiddenInGame` (`self.PointLight2`) true false)
        (elif (`/Game/Devs/Mert/Blueprints/Player/BP_PlayerCharacterMertNew.2 Loop` _asbp_player_character_mert_new)
          (`SceneComponent.SetHiddenInGame` (`self.PointLight1`) true false)
          (`SceneComponent.SetHiddenInGame` _pointlight2 false false)
          (elif (`/Game/Devs/Mert/Blueprints/Player/BP_PlayerCharacterMertNew.3 Loop` _asbp_player_character_mert_new)
            _))))
    (:`then_1`
      (if (`/Game/Devs/Mert/Blueprints/Enemies/EnemyEntity1.CanSeePlayer` (`|GetArrayItem` _outactors))
        (`LightComponent.SetLightFunctionMaterial` _pointlight2 "/Game/Devs/Oliver/Tutorial/LightFlickerMat.LightFlickerMat")
        (else
          (`LightComponent.SetLightFunctionMaterial` _pointlight2 null))))))

(fn `UserConstructionScript`)