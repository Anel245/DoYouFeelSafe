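; Interactable complaint note that opens a full note widget for reading and follows it with a dialogue widget on closing.
; Interact, if the note is not hidden or being inspected, shows the widget and flags the player as inactive and inspecting.
; A delayed polling loop then watches for the F key to call Exit.
; Exit restores the player, removes the note and displays the dialogue widget for a few seconds.
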(event `Exit`
  (`Widget.RemoveFromParent` (stale `/Game/Devs/Mert/Blueprints/Player/Interfaces/InteractionInterface.Interact` _returnvalue))
  (set `/Game/Devs/Mert/Blueprints/Player/BP_PlayerCharacterMert.IsPlayerActive` true (stale _asbp_player_character_mert))
  (set `/Game/Devs/Mert/Blueprints/Player/BP_PlayerCharacterMert.IsInspecting` false (stale _asbp_player_character_mert))
  (bind _returnvalue (`|CreateWidget` "/Game/Devs/Mert/Blueprints/Player/Widgets/W_Dialogue/Notes/W_DiaComplaint.W_DiaComplaint_C"))
  (`UserWidget.AddToViewport` _returnvalue 0)
  (`/Game/Devs/Mert/Blueprints/Player/Widgets/W_Dialogue/Notes/W_DiaComplaint.Opacity` _returnvalue)
  (`KismetSystemLibrary.Delay` 6.0)
  (`Widget.RemoveFromParent` _returnvalue))

(event `/Game/Devs/Mert/Blueprints/Player/Interfaces/InteractionInterface.Interact`
  (if (`self.bHidden`)
    _
    (elif (not (`/Game/Devs/Mert/Blueprints/Player/BP_PlayerCharacterMert.IsInspecting` (stale _asbp_player_character_mert)))
      (bind _returnvalue (`|CreateWidget` "/Game/Devs/Mert/Blueprints/Player/Widgets/W_Notes/W_NoteComplaint.W_NoteComplaint_C"))
      (`UserWidget.AddToViewport` _returnvalue 0)
      (bind _asbp_player_character_mert (cast `/Game/Devs/Mert/Blueprints/Player/BP_PlayerCharacterMert` (`GameplayStatics.GetPlayerCharacter` 0)))
      (set `/Game/Devs/Mert/Blueprints/Player/BP_PlayerCharacterMert.IsPlayerActive` false _asbp_player_character_mert)
      (set `/Game/Devs/Mert/Blueprints/Player/BP_PlayerCharacterMert.IsInspecting` true _asbp_player_character_mert)
      (`KismetSystemLibrary.Delay` 0.4)
      (if (`PlayerController.IsInputKeyDown` (`GameplayStatics.GetPlayerController` 0) "F") :!label _label
        (`self.Exit`)
        (else
          (`KismetSystemLibrary.Delay` 0.1)
          (goto _label))))))

(fn `UserConstructionScript`)