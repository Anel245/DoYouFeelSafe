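; Point light actor that switches four lights to reflect the player's loop progress and enemy sightings.
; A delayed Tick reruns the LoopChange logic, reading BP_PlayerCharacterMert's loop flags and HasHandle to show or hide the first three lights.
; Enemy/PlayerSee shows the fourth light with a flicker light-function material while the player or the first enemy or minion has sight, rechecking on a Delay and hiding it once none do.
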(event `LoopChange`
  (bind _asbp_player_character_mert (cast `/Game/Devs/Mert/Blueprints/Player/BP_PlayerCharacterMert` (`GameplayStatics.GetPlayerPawn` 0) :!label _label))
  (if (`/Game/Devs/Mert/Blueprints/Player/BP_PlayerCharacterMert.1 Loop` _asbp_player_character_mert)
    _
    (elif (`/Game/Devs/Mert/Blueprints/Player/BP_PlayerCharacterMert.2 Loop` _asbp_player_character_mert)
      (`SceneComponent.SetHiddenInGame` (`self.PointLight1`) true false)
      (`SceneComponent.SetHiddenInGame` (`self.PointLight2`) false false)
      (elif (`/Game/Devs/Mert/Blueprints/Player/BP_PlayerCharacterMert.3 Loop` _asbp_player_character_mert)
        (if (`/Game/Devs/Mert/Blueprints/Player/BP_PlayerCharacterMert.HasHandle` _asbp_player_character_mert)
          (`SceneComponent.SetHiddenInGame` (`self.PointLight1`) true false)
          (`SceneComponent.SetHiddenInGame` (`self.PointLight2`) true false)
          (`SceneComponent.SetHiddenInGame` (`self.PointLight3`) true false)
          (else
            (`SceneComponent.SetHiddenInGame` (`self.PointLight1`) true false)
            (`SceneComponent.SetHiddenInGame` (`self.PointLight2`) true false)
            (`SceneComponent.SetHiddenInGame` (`self.PointLight3`) false false)))))))

(event `self.ReceiveTick`
  (params (DeltaSeconds :type "Float (single-precision)"))
  (`KismetSystemLibrary.Delay` 0.5)
  (goto _label))

(event `Enemy/Player See`
  (bind _pointlight4 (`self.PointLight4`))
  (bind _asbp_player_character_mert (cast `/Game/Devs/Mert/Blueprints/Player/BP_PlayerCharacterMert` (`GameplayStatics.GetPlayerPawn` 0)))
  (bind _outactors (`GameplayStatics.GetAllActorsOfClass` "/Game/Devs/Mert/Blueprints/Enemies/EnemyEntity1.EnemyEntity1_C"))
  (bind _outactors_2 (`GameplayStatics.GetAllActorsOfClass` "/Game/Devs/Mert/Blueprints/Enemies/EnemyMinionEntity1.EnemyMinionEntity1_C"))
  (if (`/Game/Devs/Mert/Blueprints/Player/BP_PlayerCharacterMert.CanSeeEnemy` _asbp_player_character_mert) :!label _label_2
    (`SceneComponent.SetHiddenInGame` _pointlight4 false false :!label _label_3)
    (`LightComponent.SetLightFunctionMaterial` _pointlight4 "/Game/Devs/Oliver/Tutorial/LightFlickerMat.LightFlickerMat")
    (`KismetSystemLibrary.Delay` 0.3)
    (goto _label_2)
    (elif (`/Game/Devs/Mert/Blueprints/Enemies/EnemyEntity1.CanSeePlayer` (`|GetArrayItem` _outactors))
      (goto _label_3)
      (elif (`/Game/Devs/Mert/Blueprints/Enemies/EnemyMinionEntity1.CanSeePlayer` (`|GetArrayItem` _outactors_2))
        (goto _label_3)
        (else
          (`SceneComponent.SetHiddenInGame` _pointlight4 true false)
          (`LightComponent.SetLightFunctionMaterial` _pointlight4 null))))))

(fn `UserConstructionScript`)