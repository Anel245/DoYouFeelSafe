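; Hiding-spot actor with a creaking door that the player can hide inside, locked during loop 1 with a "no need" widget and one-time dialogue.
; Interact disables player collision, blends the view to this actor while a timeline swings the door, then hides the player and ignores look input.
; A 0.2-second delay loop polls F to trigger Exit, which reverses the door, blends back to the turned-around player and restores them.
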(event `Exit`
  (bind _playermertref (`self.PlayerMertref`))
  (bind _playermertref_2 (`self.PlayerMertref`))
  (`GameplayStatics.PlaySoundAtLocation` "/Game/Devs/Mert/Sounds/Environment/WoodCreak.WoodCreak" (`self.K2_GetActorLocation`) (struct) 0.5 (`KismetMathLibrary.RandomFloatInRange` 0.8 0.95) 0.0 null null null null)
  (set `self.Hiding` false)
  (`self.SetActorEnableCollision` _playermertref true)
  (`PlayerController.SetViewTargetWithBlend` (`GameplayStatics.GetPlayerController` 0) _playermertref 1.0 "VTBlend_Linear" 0.0 false) ; Unpossess
  (`/Game/Devs/Mert/Blueprints/Player/BP_PlayerCharacterMert.PlayerTurnAround` _playermertref)
  (`|ExecutionSequence`
    (:`then_0`
      (`KismetSystemLibrary.Delay` 1.0)
      (`self.SetActorHiddenInGame` _playermertref_2 false)
      (set `/Game/Devs/Mert/Blueprints/Player/BP_PlayerCharacterMert.IsPlayerActive` true _playermertref_2)
      (`Controller.ResetIgnoreLookInput` (`GameplayStatics.GetPlayerController` 0)))
    (:`then_1`
      (bind (_direction _door) (`Timeline|OpenCloseDoorTL` :!via `Reverse` :!label _label)
        (:`Update`
          (`SceneComponent.K2_SetRelativeRotation` (`self.Sphere5`) (`KismetMathLibrary.MakeRotator` 180.0 0.0 (`KismetMathLibrary.Lerp` (`self.CloseAngle`) (`self.OpenAngle`) _door)) false false)
          (`SceneComponent.K2_SetRelativeRotation` (`self.Sphere12`) (`KismetMathLibrary.MakeRotator` 180.0 0.0 (`KismetMathLibrary.Lerp` (`self.CloseAngle`) (`self.OpenAngle`) _door)) false false)
          (`SceneComponent.K2_SetRelativeRotation` (`self.Sphere14`) (`KismetMathLibrary.MakeRotator` 180.0 0.0 (`KismetMathLibrary.Lerp` (`self.CloseAngle`) (`self.OpenAngle`) _door)) false false))))))

(event `/Game/Devs/Mert/Blueprints/Player/Interfaces/InteractionInterface.Interact`
  (bind _returnvalue (`GameplayStatics.GetPlayerController` 0))
  (bind _playermertref (`self.PlayerMertref`))
  (bind _asbp_player_character_mert (cast `/Game/Devs/Mert/Blueprints/Player/BP_PlayerCharacterMert` (`GameplayStatics.GetPlayerCharacter` 0)))
  (bind _output_get (set `self.PlayerMertref` _asbp_player_character_mert))
  (if (`/Game/Devs/Mert/Blueprints/Player/BP_PlayerCharacterMert.1 Loop` _output_get)
    ;[1 1 1] Loop 1 can not enter
    (bind _returnvalue_2 (`|CreateWidget` "/Game/Devs/Mert/Blueprints/Player/Widgets/W_Dialogue/W_NoNeed.W_NoNeed_C"))
    (`UserWidget.AddToViewport` _returnvalue_2 0)
    (`/Game/Devs/Mert/Blueprints/Player/Widgets/W_Dialogue/W_NoNeed.Opacity` _returnvalue_2)
    (`/Engine/EditorBlueprintResources/StandardMacros.DoOnce` false
      (:`Completed`
        (`GameplayStatics.PlaySoundAtLocation` "/Game/Devs/Mert/Sounds/Player/1Loop/Dia1NoNeed.Dia1NoNeed" (`self.K2_GetActorLocation`) (struct) 0.8 1.0 0.0 null null null null)))
    (else
      (set `/Game/Devs/Mert/Blueprints/Player/BP_PlayerCharacterMert.Interacting` true _output_get)
      (if (not (`self.Hiding`))
        (`GameplayStatics.PlaySoundAtLocation` "/Game/Devs/Mert/Sounds/Environment/WoodCreak.WoodCreak" (`self.K2_GetActorLocation`) (struct) 0.5 (`KismetMathLibrary.RandomFloatInRange` 0.95 1.15) 0.0 null null null null)
        (set `self.Hiding` true)
        (`self.SetActorEnableCollision` _playermertref false)
        (set `/Game/Devs/Mert/Blueprints/Player/BP_PlayerCharacterMert.IsPlayerActive` false _playermertref)
        (`PlayerController.SetViewTargetWithBlend` (`GameplayStatics.GetPlayerController` 0) self 1.2 "VTBlend_Linear" 1.2 false) ; Possess
        (`|ExecutionSequence`
          (:`then_0`
            (goto _label))
          (:`then_1`
            (`KismetSystemLibrary.Delay` 1.0)
            (`self.SetActorHiddenInGame` (`self.PlayerMertref`) true)
            (`Controller.SetIgnoreLookInput` _returnvalue true)
            (if (`PlayerController.IsInputKeyDown` _returnvalue "F") :!label _label_2
              (`self.Exit`)
              (else
                (`KismetSystemLibrary.Delay` 0.2)
                (goto _label_2)))))))))

(fn `UserConstructionScript`)