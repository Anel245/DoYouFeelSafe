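; BP_MusicBox is a music box that plays a tutorial and reacts to hits.
; The first interaction, gated by a player character cast, plays tutorial audio, then after a delay adds the Sub_Tutorial_MusicBox widget and calls its Opacity.
; A hit plays a pickup sound at the hit location and hides the MusicBox component, using a DoOnce with a brief delayed reset to debounce repeated hits.
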(event `/Game/Devs/Mert/Blueprints/Player/Interfaces/InteractionInterface.Interact`
  ;[1 1 1] Interaction
  (`/Engine/EditorBlueprintResources/StandardMacros.DoOnce` false
    (:`Completed`
      (cast `/Game/Devs/Mert/Blueprints/Player/BP_PlayerCharacterMertNew` (`GameplayStatics.GetPlayerCharacter` 0))
      (`GameplayStatics.PlaySoundAtLocation` "/Game/Devs/Oliver/Tutorial/Audio_MusicBox_Tutorial.Audio_MusicBox_Tutorial" (0.0 0.0 0.0) (struct) 1.0 1.0 0.0 null null null null)
      (`KismetSystemLibrary.Delay` 3.0)
      (bind _returnvalue (`|CreateWidget` "/Game/Devs/Oliver/TutorialSubs/Sub_Tutorial_MusicBox.Sub_Tutorial_MusicBox_C"))
      (`UserWidget.AddToViewport` _returnvalue 0)
      (`/Game/Devs/Oliver/TutorialSubs/Sub_Tutorial_MusicBox.Opacity` _returnvalue))))

(event `self.ReceiveHit`
  (params (MyComp :type "PrimitiveComponent Object Reference") (Other :type "Actor Object Reference") (OtherComp :type "PrimitiveComponent Object Reference") (bSelfMoved :type Boolean) (HitLocation :type "Vector Structure") (HitNormal :type "Vector Structure") (NormalImpulse :type "Vector Structure") (Hit :type "HitResult Structure (by ref)"))
  ;[1 1 1] Hit Sound
  (`|ExecutionSequence`
    (:`then_0`
      (`/Engine/EditorBlueprintResources/StandardMacros.DoOnce` false :!label _label
        (:`Completed`
          (`GameplayStatics.PlaySoundAtLocation` "/Game/Devs/Mert/Sounds/Player-Footsteps/PickUp.PickUp" HitLocation (struct) 0.8 1.2 0.0 null null null null)
          (`SceneComponent.SetHiddenInGame` (`self.MusicBox`) true false))))
    (:`then_1`
      (`KismetSystemLibrary.Delay` 0.01)
      (goto _label :!via `Reset`))))

(fn `UserConstructionScript`)