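; Music box interactable that opens when used and then moves the player on to Gate_2_Scene_2.
; Interact runs a one-time timeline animating six box components, and separately consumes the player's handle if held; the opening does not require it.
; When the timeline finishes, LoadLevel plays bossfight music and a heartbeat, fades to black, clears the player's Tutorial flag and opens the level.
; MusicBox4 starts hidden; its reveal-with-sounds chain is unconnected.
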(event `LoadLevel`
  (bind _returnvalue (`GameplayStatics.CreateSound2D` "/Game/Devs/Mert/Sounds/Entity/MusicBoxBossfight.MusicBoxBossfight" 1.0 1.0 0.0 null))
  (`AudioComponent.FadeIn` _returnvalue 0.7 1.0 0.0 "Linear")
  (`KismetSystemLibrary.Delay` 5.0)
  (`GameplayStatics.PlaySound2D` "/Game/Devs/Mert/Sounds/Entity/HeartbeatSound.HeartbeatSound" 1.0 1.0 0.0 null null)
  (`KismetSystemLibrary.Delay` 2.0)
  (bind _returnvalue_2 (`|CreateWidget` "/Game/Devs/Oliver/Tutorial/TutorialSubs/W_TUT_BlackBlend.W_TUT_BlackBlend_C"))
  (`UserWidget.AddToViewport` _returnvalue_2 0)
  (`/Game/Devs/Oliver/Tutorial/TutorialSubs/W_TUT_BlackBlend.BlackTransition` _returnvalue_2)
  (`AudioComponent.FadeOut` _returnvalue 1.5 0.0 "Linear")
  (bind _asbp_player_character_mert (cast `/Game/Devs/Mert/Blueprints/Player/BP_PlayerCharacterMert` (`GameplayStatics.GetPlayerCharacter` 0)))
  (set `/Game/Devs/Mert/Blueprints/Player/BP_PlayerCharacterMert.Tutorial` false _asbp_player_character_mert)
  (`KismetSystemLibrary.Delay` 1.0)
  (`GameplayStatics.OpenLevel` "Gate_2_Scene_2"))

(event `self.ReceiveBeginPlay`
  (`SceneComponent.SetHiddenInGame` (`self.MusicBox4`) true false))

(event `/Game/Devs/Mert/Blueprints/Player/Interfaces/InteractionInterface.Interact`
  (bind _asbp_player_character_mert (cast `/Game/Devs/Mert/Blueprints/Player/BP_PlayerCharacterMert` (`GameplayStatics.GetPlayerCharacter` 0)))
  (`|ExecutionSequence`
    (:`then_0`
      (`/Engine/EditorBlueprintResources/StandardMacros.DoOnce` false
        (:`Completed`
          (bind (_direction _angle _position) (`Timeline|Timeline`)
            (:`Update`
              (`SceneComponent.K2_SetRelativeLocationAndRotation` (`self.MusicBox10`) (`KismetMathLibrary.MakeVector` 0.0 (`KismetMathLibrary.Lerp` (`self.ClosePosition`) (`self.OpenPosition`) _position)) (`KismetMathLibrary.MakeRotator` (`KismetMathLibrary.Lerp` (`self.CloseAngle`) (`self.OpenAngle`) _angle)) false false)
              (`SceneComponent.K2_SetRelativeLocationAndRotation` (`self.MusicBox30`) (`KismetMathLibrary.MakeVector` 0.0 (`KismetMathLibrary.Lerp` (`self.ClosePosition`) (`self.OpenPosition`) _position)) (`KismetMathLibrary.MakeRotator` (`KismetMathLibrary.Lerp` (`self.CloseAngle`) (`self.OpenAngle`) _angle)) false false)
              (`SceneComponent.K2_SetRelativeLocationAndRotation` (`self.MusicBox25`) (`KismetMathLibrary.MakeVector` 0.0 (`KismetMathLibrary.Lerp` (`self.ClosePosition`) (`self.OpenPosition`) _position)) (`KismetMathLibrary.MakeRotator` (`KismetMathLibrary.Lerp` (`self.CloseAngle`) (`self.OpenAngle`) _angle)) false false)
              (`SceneComponent.K2_SetRelativeLocationAndRotation` (`self.MusicBox26`) (`KismetMathLibrary.MakeVector` 0.0 (`KismetMathLibrary.Lerp` (`self.ClosePosition`) (`self.OpenPosition`) _position)) (`KismetMathLibrary.MakeRotator` (`KismetMathLibrary.Lerp` (`self.CloseAngle`) (`self.OpenAngle`) _angle)) false false)
              (`SceneComponent.K2_SetRelativeLocationAndRotation` (`self.MusicBox27`) (`KismetMathLibrary.MakeVector` 0.0 (`KismetMathLibrary.Lerp` (`self.ClosePosition`) (`self.OpenPosition`) _position)) (`KismetMathLibrary.MakeRotator` (`KismetMathLibrary.Lerp` (`self.CloseAngle`) (`self.OpenAngle`) _angle)) false false)
              (`SceneComponent.K2_SetRelativeLocationAndRotation` (`self.MusicBox28`) (`KismetMathLibrary.MakeVector` 0.0 (`KismetMathLibrary.Lerp` (`self.ClosePosition`) (`self.OpenPosition`) _position)) (`KismetMathLibrary.MakeRotator` (`KismetMathLibrary.Lerp` (`self.CloseAngle`) (`self.OpenAngle`) _angle)) false false))
            (:`Finished`
              (`self.LoadLevel`))))))
    (:`then_1`
      (if (`/Game/Devs/Mert/Blueprints/Player/BP_PlayerCharacterMert.HasHandle` _asbp_player_character_mert)
        (set `/Game/Devs/Mert/Blueprints/Player/BP_PlayerCharacterMert.Interacting` true _asbp_player_character_mert)
        (set `/Game/Devs/Mert/Blueprints/Player/BP_PlayerCharacterMert.HasHandle` false _asbp_player_character_mert)))))

(fn `UserConstructionScript`)