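; BP_PlayerCharacterOli is a player character Blueprint with pistol reloading and footstep audio.
; PistolReload refills a non-full clip from reserve ammo, deducting a whole clip regardless of rounds left, or loading the remaining reserve when it is short.
; FootstepTry plays a wooden footstep cue when a capsule-radius sphere trace toward the feet hits and the character has velocity.
; Interact and the construction script are empty.
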(fn `FootstepTrace`
  (returns (ReturnValue :type Boolean))
  (bind _returnvalue (`self.K2_GetActorLocation`))
  (bind _capsulecomponent (`self.CapsuleComponent`))
  (bind (_x _y _z) (`KismetMathLibrary.BreakVector3f` _returnvalue))
  (bind (_outhit _returnvalue_2) (`KismetSystemLibrary.SphereTraceSingle` _returnvalue (`KismetMathLibrary.MakeVector` _x _y (- _z (`CapsuleComponent.GetScaledCapsuleHalfHeight` _capsulecomponent))) (`CapsuleComponent.GetScaledCapsuleRadius` _capsulecomponent) "TraceTypeQuery1"))
  (return _returnvalue_2))

(fn `FootstepTry`
  (bind _returnvalue (`self.FootstepTrace`))
  (if _returnvalue
    (if (> (`KismetMathLibrary.VSize` (`self.GetVelocity`)) 0.0)
      (`GameplayStatics.PlaySoundAtLocation` "/Game/Devs/Mert/Sounds/Player-Footsteps/WoodenFootstep_Cue.WoodenFootstep_Cue" (`self.K2_GetActorLocation`) (struct) 1.0 1.0 0.0 "/Game/Devs/Mert/Sounds/Player/PlayerAttenuation.PlayerAttenuation" null null null))))

(fn `Interact`)

(fn `PistolReload`
  (if (== (`self.PistolAmmo`) (`self.PistolClipSize`))
    _
    (elif (> (`self.PistolMaxAmmo`) (`self.PistolClipSize`))
      (set `self.PistolAmmo` (`self.PistolClipSize`))
      (set `self.PistolMaxAmmo` (- (`self.PistolMaxAmmo`) (`self.PistolClipSize`)))
      (else
        (set `self.PistolAmmo` (`self.PistolMaxAmmo`))
        (set `self.PistolMaxAmmo` 0)))))

(fn `UserConstructionScript`)